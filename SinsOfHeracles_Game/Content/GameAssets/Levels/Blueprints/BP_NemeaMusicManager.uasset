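; BP_NemeaMusicManager is a music manager, apparently for the Nemea level, that also starts a wind sound when its trigger event fires.
; PushMusic and PopMusic edit a track array used as a priority stack, then call SwitchMusic.
; SwitchMusic crossfades to a newly spawned 2D sound of the last track, or PlainMusic when empty, after comparing against CurrentMusic, which these graphs never update.
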(event Custom|TriggerWind
  (Audio|Components|Audio|Play (Variables|Components|GetWindSoundRef) 2.0))

(event EventBeginPlay
  (EventDispatchers|BindEventtoOnTriggerWind (delegate Custom|TriggerWind)))

(fn ConstructionScript)

(fn SwitchMusic
  (bind _musicarray (Variables|Default|GetMusicArray))
  (bind _currentmusic (Variables|Default|GetCurrentMusic))
  (bind _returnvalue (Utilities|Array|LastIndex _musicarray))
  (bind _output (Utilities|Array|Get(acopy) _musicarray _returnvalue))
  (bind _returnvalue_2 (== _currentmusic _output))
  (if (Utilities|Array|IsValidIndex (Variables|Default|GetMusicArray))
    (if (not _returnvalue_2)
      (Audio|Components|Audio|FadeOut (Variables|Components|GetAudio) 2.0 0.0 "Linear" :!class /Script/Engine.AudioComponent)
      (bind _returnvalue_3 (Audio|SpawnSound2D _output 3.0 1.0 0.0 0))
      (bind _output_get (Variables|Components|SetAudio _returnvalue_3))
      (Audio|Components|Audio|FadeIn _output_get 1.0 1.0 0.0 "Linear" :!class /Script/Engine.AudioComponent))
    (elif _returnvalue_2
      (Audio|Components|Audio|FadeOut (Variables|Components|GetAudio) 2.0 0.0 "Linear" :!class /Script/Engine.AudioComponent)
      (bind _returnvalue_4 (Audio|SpawnSound2D "/Game/GameAssets/Assets/Musics/plainMusic.plainMusic" 3.0 1.0 0.0 0))
      (bind _output_get_2 (Variables|Components|SetAudio _returnvalue_4))
      (Audio|Components|Audio|FadeIn _output_get_2 1.0 1.0 0.0 "Linear" :!class /Script/Engine.AudioComponent))))

(fn PushMusic
  (params (NewMusic :type Sound%20Base%20Object%20Reference))
  (Utilities|Array|Add (Variables|Default|GetMusicArray) NewMusic)
  (CallFunction|SwitchMusic))

(fn PopMusic
  (params (TrackToRemove :type Sound%20Base%20Object%20Reference))
  (Utilities|Array|RemoveItem (Variables|Default|GetMusicArray) TrackToRemove)
  (CallFunction|SwitchMusic))