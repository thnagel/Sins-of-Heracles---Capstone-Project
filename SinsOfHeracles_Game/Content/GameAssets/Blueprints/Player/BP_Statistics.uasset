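; BP_Statistics tracks the player's Vitality and Endurance stats and applies their increases to the player character.
; On BeginPlay it casts player character 0 to BP_Player and caches the reference.
; IncreaseVitality adds the given amount to Vitality and to the player's max and current Health.
; IncreaseEndurance does the same for Endurance and the player's max and current Stamina.
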(event EventBeginPlay
  (bind _asbp_player (Utilities|Casting|CastToBP_Player (Game|GetPlayerCharacter 0)))
  (Variables|Default|SetPlayer _asbp_player))

(fn ConstructionScript)

(fn IncreaseVitality
  (params (Ammount%20to%20increase%20by :type Integer))
  (bind _player (Variables|Default|GetPlayer))
  (Variables|Default|SetVitality (+ Ammount%20to%20increase%20by (Variables|Default|GetVitality)))
  (Variables|/Game/GameAssets/Blueprints/Player/BP_Player.BP_Player_C|SetMaxHealth _player (+ (Variables|/Game/GameAssets/Blueprints/Player/BP_Player.BP_Player_C|GetMaxHealth _player) Ammount%20to%20increase%20by))
  (Variables|/Game/GameAssets/Blueprints/Player/BP_Player.BP_Player_C|SetHealth _player (+ Ammount%20to%20increase%20by (Variables|/Game/GameAssets/Blueprints/Player/BP_Player.BP_Player_C|GetHealth _player))))

(fn IncreaseEndurance
  (params (Ammount%20to%20increase%20by :type Integer))
  (bind _player (Variables|Default|GetPlayer))
  (Variables|Default|SetEndurance (+ Ammount%20to%20increase%20by (Variables|Default|GetEndurance)))
  (Variables|/Game/GameAssets/Blueprints/Player/BP_Player.BP_Player_C|SetMaxStamina _player (+ (Variables|/Game/GameAssets/Blueprints/Player/BP_Player.BP_Player_C|GetMaxStamina _player) Ammount%20to%20increase%20by))
  (Variables|/Game/GameAssets/Blueprints/Player/BP_Player.BP_Player_C|SetStamina _player (+ Ammount%20to%20increase%20by (Variables|/Game/GameAssets/Blueprints/Player/BP_Player.BP_Player_C|GetStamina _player))))