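; BP_GruntRanged is a ranged enemy that shoots arrows at the player, with AI-facing getters for health, patrol route, range and speed setting.
; Attack plays a draw montage, then launches BP_Arrow toward the player's spine socket.
; Hits reduce health, update a camera-facing health bar, play pain feedback and report player-caused damage to AI perception after the impact montage.
; A separate event ragdolls the body on death.
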(event Custom|Fire%20Arrow
  (params (Target :type Actor%20Object%20Reference))
  (bind _as_bp_player (Variables|Default|GetAs%20BP%20Player))
  (bind _arrow_spawn_point (Variables|Default|GetArrow%20spawn%20point))
  (bind _returnvalue (Transformation|GetWorldLocation _arrow_spawn_point))
  (bind _mesh (Variables|/Script/Engine.Character|GetMesh _as_bp_player))
  (bind _returnvalue_2 (Transformation|GetSocketLocation _mesh "spine_05"))
  (bind _returnvalue_3 (- _returnvalue_2 _returnvalue))
  (bind _returnvalue_4 (Math|Vector|Normalize _returnvalue_3))
  (bind _returnvalue_5 (Math|Rotator|MakeRotfromX _returnvalue_4))
  ;[0.15 0.15 0.15 0.5] Fire Arrow
  (bind _returnvalue_6 (Game|SpawnActorfromClass "/Game/GameAssets/Blueprints/Enemies/GruntRanged/BP_Arrow.BP_Arrow_C" (Math|Transform|MakeTransform (Transformation|GetWorldLocation (Variables|Default|GetArrow%20spawn%20point)) _returnvalue_5 "1.000000,1.000000,1.000000") "Undefined" "MultiplyWithRoot" 0 0))
  (bind _output_get (Variables|Default|SetSpawnedArrow _returnvalue_6))
  (Variables|/Script/Engine.MovementComponent|SetVelocity (Variables|/Game/GameAssets/Blueprints/Enemies/GruntRanged/BP_Arrow.BP_Arrow_C|GetProjectileMovement _output_get) (* (Math|Vector|GetForwardVector _returnvalue_5) 4e+03)))

(event EventApplyDamage
  (params (AttackDamage :type Integer))
  ;[0.15 0.15 0.15 0.5] Apply Damage
  (Variables|Default|SetPreviousHealth (Variables|Default|GetHealth))
  (Variables|Default|SetHealth (- (Variables|Default|GetHealth) AttackDamage))
  (CallFunction|UpdateHealthBarValues false)
  (Components|Timeline|PlayfromStart (Variables|Default|GetHealthSmoothUI))
  (Audio|PlaySoundatLocation (.OutItem (Utilities|Array|Random (Variables|Default|GetPainGrunts))) (Transformation|GetActorLocation) "0, 0, 0" 1.0 (Math|Random|RandomFloatinRange 0.8 1.0) 0.0 "/Game/GameAssets/Blueprints/Enemies/GruntMelee/SA_Grunt.SA_Grunt" 0 0 0)
  (Animation|Montage|PlayMontage (Variables|Character|GetMesh) "/Game/GameAssets/Assets/Mixamo/Animations/Sword_And_Shield/Manny/RootMotionned/AM_sword_impact_3.AM_sword_impact_3"
    (:OnCompleted
      (if (Variables|Default|GetPlayerhit)
        (Class|AISenseDamage|ReportDamageEvent self (Game|GetPlayerCharacter 0) (Math|Conversions|ToFloat(Integer) (Variables|Default|GetAttack%20Damage)) (Transformation|GetActorLocation) "0, 0, 0" "None")))))

(event EventBeginPlay
  (CallFunction|InitHealthBar))

(event EventResolveAttack
  (params (AttackingActor :type Actor%20Object%20Reference) (AttackLocation :type Vector :default "0, 0, 0") (AttackDamage :type Integer))
  ;[0.15 0.15 0.15 0.5] Resolve Attack
  (if (== AttackingActor (Game|GetPlayerCharacter 0))
    (Variables|Default|SetPlayerhit true))
  (bind _output_get (Variables|Default|SetAttack%20Damage AttackDamage))
  (CallFunction|ApplyDamage _output_get))

(event EventTick
  (params (DeltaSeconds :type Float%20%28single-precision%29))
  ;[0.15 0.15 0.15 0.5] Event tick
  (CallFunction|UpdateHealthBarRotation))

(event EventAttack
  (params (TargetActor :type Actor%20Object%20Reference))
  ;[0.15 0.15 0.15 0.5] Attack
  (bind _asbp_player (Utilities|Casting|CastToBP_Player TargetActor))
  (Variables|Default|SetAs%20BP%20Player _asbp_player)
  (if (not (Variables|Default|GetIsAttacking))
    (Variables|Default|SetAttackAnim "/Game/GameAssets/Blueprints/Enemies/GruntRanged/Animations/standing_draw_arrow1_Montage.standing_draw_arrow1_Montage")
    (Animation|Montage|PlayMontage (Variables|Character|GetMesh) (Variables|Default|GetAttackAnim)
      (:then
        (Audio|PlaySoundatLocation "/Game/GameAssets/Assets/SFX/Enemies/RangedGrunt/ArrowRelease.ArrowRelease" (Transformation|GetActorLocation) "0, 0, 0" 7.0 (Math|Random|RandomFloatinRange 0.8 1.0) 0.0 "/Game/GameAssets/Blueprints/Enemies/GruntMelee/SA_Grunt.SA_Grunt" 0 0 0))
      (:OnCompleted
        (CallFunction|FireArrow TargetActor)))))

(event EventDeathRagdoll
  (bind _mesh (Variables|Character|GetMesh))
  ;[0.15 0.15 0.15 0.5] Death Ragdoll
  (Pawn|Components|CharacterMovement|DisableMovement (Variables|Character|GetCharacterMovement))
  (Collision|SetCollisionEnabled (Variables|Collision|GetCapsuleComponent) "NoCollision")
  (Physics|SetSimulatePhysics _mesh true)
  (Collision|SetCollisionProfileName _mesh "Ragdoll" true :!class /Script/Engine.PrimitiveComponent))

(fn ConstructionScript)

(fn UpdateHealthBarValues
  (params (IsLockedByPlayer :type Boolean))
  (bind _as_wbp_enemy_health_bar (Variables|Default|GetAs%20WBP%20Enemy%20Health%20Bar))
  ;[0.15 0.15 0.15 0.5] Set Percentage
  (Progress|SetPercent (Variables|/Game/GameAssets/Blueprints/Enemies/UI/WBP_EnemyHealthBar.WBP_EnemyHealthBar_C|GetHealthBar (Variables|Default|GetAs%20WBP%20Enemy%20Health%20Bar)) (/ (Variables|Default|GetHealth) (Variables|Default|GetMaxHealth)))
  ;[0.15 0.15 0.15 0.5] Set Visibility
  (if (> (Variables|Default|GetHealth) 0)
    (if IsLockedByPlayer
      (Widget|SetVisibility (Variables|Default|GetAs%20WBP%20Enemy%20Health%20Bar) "Visible")
      (elif (< (Variables|Default|GetHealth) (Variables|Default|GetMaxHealth))
        (Widget|SetVisibility _as_wbp_enemy_health_bar "Visible")
        (else
          (Widget|SetVisibility _as_wbp_enemy_health_bar "Hidden"))))
    (else
      (Widget|SetVisibility (Variables|Default|GetAs%20WBP%20Enemy%20Health%20Bar) "Hidden"))))

(fn UpdateHealthBarRotation
  (bind _w_healthbar (Variables|Default|GetW_HealthBar))
  (Transformation|SetWorldRotation _w_healthbar (Math|Rotator|FindLookatRotation (Transformation|GetWorldLocation _w_healthbar) (Transformation|GetWorldLocation (Variables|/Script/Engine.PlayerCameraManager|GetTransformComponent (Game|GetPlayerCameraManager 0)))) false false))

(fn InitHealthBar
  (bind _aswbp_enemy_health_bar (Utilities|Casting|CastToWBP_EnemyHealthBar (UserInterface|GetWidget (Variables|Default|GetW_HealthBar))))
  (Variables|Default|SetAs%20WBP%20Enemy%20Health%20Bar _aswbp_enemy_health_bar)
  (CallFunction|UpdateHealthBarValues false)
  (CallFunction|UpdateHealthBarRotation))

(fn GetCurrentHealth
  (return (Variables|Default|GetHealth)))

(fn GetIdealRange
  (return 0.0 0.0))

(fn GetPatrolRoute
  (return (Variables|Default|GetPatrolRoute)))

(fn SetMovementSpeed
  (params (Speed :type E_AIMovementSpeed%20Enum :default "NewEnumerator0"))
  (bind _output_get (Variables|/Script/Engine.CharacterMovementComponent|SetMaxWalkSpeed (Variables|Character|GetCharacterMovement) (Utilities|Select :Index Speed :NewEnumerator0 0.0 :NewEnumerator1 1e+02 :NewEnumerator2 3e+02 :NewEnumerator3 5e+02)))
  (return _output_get))