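; BP_Arrow is a ranged Grunt enemy projectile that damages the player on contact.
; A mesh overlap with the player sends an attack message with fixed damage, then destroys the arrow after a short delay.
; A separate radius overlap plays a one-time, pitch-randomized swish when the arrow hits or passes near the player.
; A lifespan set on BeginPlay cleans up arrows that never hit.
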(event OnComponentBeginOverlap(SFXradius)
  (params (OverlappedComponent :type Primitive%20Component%20Object%20Reference) (OtherActor :type Actor%20Object%20Reference) (OtherComp :type Primitive%20Component%20Object%20Reference) (OtherBodyIndex :type Integer) (bFromSweep :type Boolean) (SweepResult :type Hit%20Result%20Structure%20%28by%20ref%29))
  ;[0.15 0.15 0.15 0.5] SFX when hit or close
  (if (== OtherActor (Game|GetPlayerCharacter 0))
    (Utilities|Casting|CastToBP_Player OtherActor)
    (if (not (Variables|Default|GetWooshPlayed))
      (Variables|Default|SetWooshPlayed true)
      (Audio|PlaySoundatLocation "/Game/GameAssets/Assets/SFX/Enemies/RangedGrunt/ArrowSwish.ArrowSwish" (Transformation|GetActorLocation self) "0, 0, 0" 0.2 (Math|Random|RandomFloatinRange 0.8 1.2) 0.0 0 0 0 0))))

(event OnComponentBeginOverlap(StaticMesh)
  (params (OverlappedComponent :type Primitive%20Component%20Object%20Reference) (OtherActor :type Actor%20Object%20Reference) (OtherComp :type Primitive%20Component%20Object%20Reference) (OtherBodyIndex :type Integer) (bFromSweep :type Boolean) (SweepResult :type Hit%20Result%20Structure%20%28by%20ref%29))
  ;[0.15 0.15 0.15 0.5] Arrow damage
  (if (== OtherActor (Game|GetPlayerCharacter 0))
    (Class|BPICombatant|ResolveAttack(Message) OtherActor self (Transformation|GetActorLocation) 5)
    (Utilities|FlowControl|Delay 0.1)
    (Actor|DestroyActor)))

(event EventBeginPlay
  ;[0.15 0.15 0.15 0.5] Set Max duration in case it never hits
  (Actor|SetLifeSpan 3e+01))

(fn ConstructionScript)