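; Melee grunt enemy character with health, ragdoll death, and range, patrol and speed functions.
; Attack montage notifies open a window for fist hitbox overlaps, using a hit list to damage each actor once per swing.
; Incoming damage updates a camera-facing health bar and plays a hit reaction; on completion it reports player-caused damage to AI perception and asks AIC_GruntMelee to check death.
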(event OnComponentBeginOverlap(FistHitbox)
  (params (OverlappedComponent :type Primitive%20Component%20Object%20Reference) (OtherActor :type Actor%20Object%20Reference) (OtherComp :type Primitive%20Component%20Object%20Reference) (OtherBodyIndex :type Integer) (bFromSweep :type Boolean) (SweepResult :type Hit%20Result%20Structure%20%28by%20ref%29))
  ;[0.15 0.15 0.15 0.5] TEMP hit detection
  (if (and (!= OtherActor self) (Variables|Default|GetIsAttacking))
    (bind _isalreadyhit (CallFunction|IsActorAlreayHit OtherActor))
    (if (not _isalreadyhit)
      (Class|BPICombatant|ResolveAttack(Message) OtherActor self (Transformation|GetWorldLocation (Variables|Default|GetFistHitbox)) 15))))

(event EventBeginPlay
  (CallFunction|InitHealthBar))

(event EventAttack
  (params (TargetActor :type Actor%20Object%20Reference))
  ;[0.15 0.15 0.15 0.5] Attack
  (if (not (Variables|Default|GetIsAttacking))
    (Variables|Default|SetAttackAnim "/Game/GameAssets/Blueprints/Enemies/GruntMelee/AM_Attack1.AM_Attack1")
    (Animation|Montage|PlayMontage (Variables|Character|GetMesh) (Variables|Default|GetAttackAnim)
      (:then
        (Audio|PlaySoundatLocation (.OutItem (Utilities|Array|Random (Variables|Default|GetAttackSFX))) (Transformation|GetActorLocation) "0, 0, 0" 1.0 1.0 0.0 "/Game/GameAssets/Blueprints/Enemies/GruntMelee/SA_Grunt.SA_Grunt" 0 0 0))
      (:OnInterrupted
        (Variables|Default|SetIsAttacking false :!label _label)
        (Utilities|Array|Clear (Variables|Default|GetHitEnnemiesList)))
      (:OnNotifyBegin
        (Variables|Default|SetIsAttacking true)
        (Audio|PlaySoundatLocation "/Game/GameAssets/Blueprints/Enemies/SFX/fist-punch-or-kick-7171.fist-punch-or-kick-7171" (Transformation|GetActorLocation) "0, 0, 0" 1.0 1.0 0.0 "/Game/GameAssets/Blueprints/Enemies/GruntMelee/SA_Grunt.SA_Grunt" 0 0 0))
      (:OnNotifyEnd
        (goto _label)))))

(event EventTick
  (params (DeltaSeconds :type Float%20%28single-precision%29))
  ;[0.15 0.15 0.15 0.5] Event tick
  (CallFunction|UpdateHealthBarRotation))

(event EventDeathRagdoll
  (bind _mesh (Variables|Character|GetMesh))
  ;[0.15 0.15 0.15 0.5] Death Ragdoll
  (Pawn|Components|CharacterMovement|DisableMovement (Variables|Character|GetCharacterMovement))
  (Collision|SetCollisionEnabled (Variables|Collision|GetCapsuleComponent) "NoCollision")
  (Physics|SetSimulatePhysics _mesh true)
  (Collision|SetCollisionProfileName _mesh "Ragdoll" true :!class /Script/Engine.PrimitiveComponent))

(event EventResolveAttack
  (params (AttackingActor :type Actor%20Object%20Reference) (AttackLocation :type Vector :default "0, 0, 0") (AttackDamage :type Integer))
  (if (== AttackingActor (Game|GetPlayerCharacter 0))
    (Variables|Default|SetPlayerHit true))
  (bind _output_get (Variables|Default|SetAttack%20Damage AttackDamage))
  (CallFunction|ApplyDamage _output_get))

(event EventApplyDamage
  (params (AttackDamage :type Integer))
  ;[0.15 0.15 0.15 0.5] Apply damage
  (Variables|Default|SetPreviousHealth (Variables|Default|GetHealth))
  (Variables|Default|SetHealth (- (Variables|Default|GetHealth) AttackDamage))
  (CallFunction|UpdateHealthBarValues false)
  (Components|Timeline|PlayfromStart (Variables|Default|GetHealthSmoothUI))
  (Audio|PlaySoundatLocation (.OutItem (Utilities|Array|Random (Variables|Default|GetPainGrunts))) (Transformation|GetActorLocation) "0, 0, 0" 1.0 (Math|Random|RandomFloatinRange 0.8 1.0) 0.0 "/Game/GameAssets/Blueprints/Enemies/GruntMelee/SA_Grunt.SA_Grunt" 0 0 0)
  (Animation|Montage|PlayMontage (Variables|Character|GetMesh) "/Game/GameAssets/Assets/Mixamo/Animations/Sword_And_Shield/Manny/RootMotionned/AM_sword_impact_3.AM_sword_impact_3"
    (:OnCompleted
      (if (Variables|Default|GetPlayerHit)
        (Class|AISenseDamage|ReportDamageEvent self (Game|GetPlayerCharacter 0) (Math|Conversions|ToFloat(Integer) (Variables|Default|GetAttack%20Damage)) (Transformation|GetActorLocation) "0, 0, 0" "None"))
      (bind _asaic_grunt_melee (Utilities|Casting|CastToAIC_GruntMelee (AI|GetAIController self)))
      (Default|CheckDeath _asaic_grunt_melee))))

(fn ConstructionScript)

(fn IsActorAlreayHit
  (params (HitActor :type Actor%20Object%20Reference))
  (for _array_element (Variables|Default|GetHitEnnemiesList)
    (if (== HitActor _array_element)
      (return true)))
  (Utilities|Array|Add (Variables|Default|GetHitEnnemiesList) HitActor)
  (return false))

(fn UpdateHealthBarValues
  (params (IsLockedByPlayer :type Boolean))
  (bind _as_wbp_enemy_health_bar (Variables|Default|GetAs%20WBP%20Enemy%20Health%20Bar))
  ;[0.15 0.15 0.15 0.5] Set Percentage
  (Progress|SetPercent (Variables|/Game/GameAssets/Blueprints/Enemies/UI/WBP_EnemyHealthBar.WBP_EnemyHealthBar_C|GetHealthBar (Variables|Default|GetAs%20WBP%20Enemy%20Health%20Bar)) (/ (Variables|Default|GetHealth) (Variables|Default|GetMaxHealth)))
  ;[0.15 0.15 0.15 0.5] Set Visibility
  (if (> (Variables|Default|GetHealth) 0)
    (if IsLockedByPlayer
      (Widget|SetVisibility (Variables|Default|GetAs%20WBP%20Enemy%20Health%20Bar) "Visible")
      (elif (< (Variables|Default|GetHealth) (Variables|Default|GetMaxHealth))
        (Widget|SetVisibility _as_wbp_enemy_health_bar "Visible")
        (else
          (Widget|SetVisibility _as_wbp_enemy_health_bar "Hidden"))))
    (else
      (Widget|SetVisibility (Variables|Default|GetAs%20WBP%20Enemy%20Health%20Bar) "Hidden"))))

(fn InitHealthBar
  (bind _aswbp_enemy_health_bar (Utilities|Casting|CastToWBP_EnemyHealthBar (UserInterface|GetWidget (Variables|Default|GetW_HealthBar))))
  (Variables|Default|SetAs%20WBP%20Enemy%20Health%20Bar _aswbp_enemy_health_bar)
  (CallFunction|UpdateHealthBarValues false))

(fn UpdateHealthBarRotation
  (bind _w_healthbar (Variables|Default|GetW_HealthBar))
  (Transformation|SetWorldRotation _w_healthbar (Math|Rotator|FindLookatRotation (Transformation|GetWorldLocation _w_healthbar) (Transformation|GetWorldLocation (Variables|/Script/Engine.PlayerCameraManager|GetTransformComponent (Game|GetPlayerCameraManager 0)))) false false))

(fn GetCurrentHealth
  (return (Variables|Default|GetHealth)))

(fn GetIdealRange
  (return 1e+02 3.5e+02))

(fn GetPatrolRoute
  (return (Variables|AI|GetPatrolRoute)))

(fn SetMovementSpeed
  (params (Speed :type E_AIMovementSpeed%20Enum :default "NewEnumerator0"))
  (bind _output_get (Variables|/Script/Engine.CharacterMovementComponent|SetMaxWalkSpeed (Variables|Character|GetCharacterMovement) (Utilities|Select :Index Speed :NewEnumerator0 0.0 :NewEnumerator1 1e+02 :NewEnumerator2 3e+02 :NewEnumerator3 5e+02)))
  (return _output_get))