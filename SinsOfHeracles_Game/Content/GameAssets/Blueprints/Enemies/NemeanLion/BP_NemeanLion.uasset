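; Nemean Lion boss enemy that fights the player, driven by AI through blackboard State and TargetActor keys.
; Dash and bite montages open a damage window in which mesh overlaps deal a single hit via combatant messages, and incoming attacks reduce its health.
; Flag-setting movement events drive strafing and walking input on Tick, which also updates a camera-facing health bar and prints state and player-distance debug text.
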(event OnComponentBeginOverlap(Mesh)
  (params (OverlappedComponent :type Primitive%20Component%20Object%20Reference) (OtherActor :type Actor%20Object%20Reference) (OtherComp :type Primitive%20Component%20Object%20Reference) (OtherBodyIndex :type Integer) (bFromSweep :type Boolean) (SweepResult :type Hit%20Result%20Structure%20%28by%20ref%29))
  ;[0.15 0.15 0.15 0.5] Overlap Event Damage
  (if (and (Variables|Default|GetIsAttacking) (not (Variables|Default|GetAlreadyHit)))
    (Variables|Default|SetAlreadyHit true)
    (Class|BPICombatant|ResolveAttack(Message) OtherActor self "0, 0, 0" 20)))

(event Custom|StartFight
  (params (TargetActor :type Actor%20Object%20Reference))
  ;[0.15 0.15 0.15 0.5] State Events
  (AI|Components|Blackboard|SetValueasObject (AI|GetBlackboard 0) (Utilities|Name|MakeLiteralName "TargetActor") TargetActor)
  (CallFunction|UpdateState "NewEnumerator1"))

(event Custom|BiteAttack
  ;[0.15 0.15 0.15 0.5] Attack Events
  (Variables|Default|SetIsAttacking true)
  (Variables|Default|SetAlreadyHit false)
  (Animation|Montage|PlayMontage (Variables|Character|GetMesh) "/Game/GameAssets/Blueprints/Enemies/NemeanLion/Animations/Reworked_Animations/AM_Lion_Bite.AM_Lion_Bite"
    (:OnCompleted
      _)
    (:OnInterrupted
      _))
  (Variables|Default|SetIsAttacking false)
  (Variables|Default|SetAlreadyHit false))

(event Custom|UpdateState
  (params (NewParam :type E_BossState%20Enum :default "NewEnumerator0"))
  ;[0.15 0.15 0.15 0.5] State Events
  (AI|Components|Blackboard|SetValueasEnum (AI|GetBlackboard 0) (Utilities|Name|MakeLiteralName "State") NewParam))

(event Custom|StartStrafing
  (params (Direction :type Vector))
  ;[0.15 0.15 0.15 0.5] Movement Events
  (if (and (not (Variables|Default|GetStrafeLeft)) (not (Variables|Default|GetStrafeRight)))
    (if (Utilities|Operators|EqualEqual Direction (Class|KismetMathLibrary|VectorRight) 0.0)
      (Variables|Default|SetStrafeRight true)
      (else
        (Variables|Default|SetStrafeLeft true)))))

(event Custom|StopStrafing
  ;[0.15 0.15 0.15 0.5] Movement Events
  (Variables|Default|SetStrafeRight false)
  (Variables|Default|SetStrafeLeft false))

(event Custom|DashOnPlayer
  ;[0.15 0.15 0.15 0.5] Attack Events
  (Variables|Default|SetIsAttacking true)
  (Variables|Default|SetAlreadyHit false)
  (Animation|Montage|PlayMontage (Variables|Character|GetMesh) "/Game/GameAssets/Blueprints/Enemies/NemeanLion/Animations/Reworked_Animations/AM_Lion_JumpAttack_RM.AM_Lion_JumpAttack_RM" 0.9
    (:OnCompleted
      _)
    (:OnInterrupted
      _))
  (Variables|Default|SetIsAttacking false)
  (Variables|Default|SetAlreadyHit false))

(event Custom|StopWalking
  ;[0.15 0.15 0.15 0.5] Movement Events
  (Variables|Default|SetWalkForward false))

(event Custom|StartWalking
  ;[0.15 0.15 0.15 0.5] Movement Events
  (Variables|Default|SetWalkForward true))

(event Custom|LionRoar
  ;[0.15 0.15 0.15 0.5] Movement Events
  (Animation|Montage|PlayMontage (Variables|Character|GetMesh) "/Game/GameAssets/Blueprints/Enemies/NemeanLion/Animations/Reworked_Animations/AM_Lion_Roar.AM_Lion_Roar" 0.75))

(event EventResolveAttack
  (params (AttackingActor :type Actor%20Object%20Reference) (AttackLocation :type Vector :default "0, 0, 0") (AttackDamage :type Integer))
  ;[0.15 0.15 0.15 0.5] BPI Combatant Event Implementation
  (Class|BPICombatant|ApplyDamage(Message) self AttackDamage))

(event EventBeginPlay
  ;[0.15 0.15 0.15 0.5] Event BeginPlay
  (CallFunction|InitHealthBar))

(event EventApplyDamage
  (params (AttackDamage :type Integer))
  ;[0.15 0.15 0.15 0.5] BPI Combatant Event Implementation
  (Variables|Default|SetHealth (- (Variables|Default|GetHealth) AttackDamage)))

(event EventTick
  (params (DeltaSeconds :type Float%20%28single-precision%29))
  ;[0.15 0.15 0.15 0.5] Event Tick
  (Utilities|FlowControl|Sequence
    (:then_0
      ;;[0.15 0.15 0.15 0.5] Strafe Movement
      (Utilities|FlowControl|Sequence
        (:then_0
          (if (Variables|Default|GetStrafeRight)
            (Class|PawnMovementComponent|AddInputVector (Variables|Character|GetCharacterMovement) (* (Math|Vector|GetRightVector (Transformation|GetActorRotation)) (Variables|Default|GetStrafeSpeedMultiplier)) true)))
        (:then_1
          (if (Variables|Default|GetStrafeLeft)
            (Class|PawnMovementComponent|AddInputVector (Variables|Character|GetCharacterMovement) (* (* (Math|Vector|GetRightVector (Transformation|GetActorRotation)) (Math|Float|MakeLiteralFloat -1.0)) (Variables|Default|GetStrafeSpeedMultiplier)) true)))))
    (:then_1
      ;;[0.15 0.15 0.15 0.5] Walking Movement
      (if (Variables|Default|GetWalkForward)
        (Class|PawnMovementComponent|AddInputVector (Variables|Character|GetCharacterMovement) (* (Math|Vector|GetForwardVector (Transformation|GetActorRotation)) (Variables|Default|GetWalkSpeedMultiplier)) true)))
    (:then_2
      ;;[0.15 0.15 0.15 0.5] Update Health Bar Value/Rotation
      (CallFunction|UpdateHealthBar))
    (:then_3
      ;[0.15 0.15 0.15 0.5] Debug Prints
      (Utilities|FlowControl|Sequence
        (:then_0
          (Development|PrintString (Utilities|String|EnumtoString (Utilities|Enum|ByteToEnumE_BossState (Class|BlackboardComponent|GetValueasEnum (AI|GetBlackboard 0) (Utilities|Name|MakeLiteralName "State")))) true true "(R=0.000000,G=0.660000,B=1.000000,A=1.000000)" 0.0))
        (:then_1
          (bind _returnvalue (Actor|GetActorOfClass "/Game/GameAssets/Blueprints/Player/BP_Player.BP_Player_C"))
          (Development|PrintString (Utilities|String|ToString(Float) (Math|Vector|VectorLength (- (Transformation|GetActorLocation _returnvalue) (Transformation|GetActorLocation)))) true true "(R=0.000000,G=0.660000,B=1.000000,A=1.000000)" 0.0))))))

(fn ConstructionScript)

(fn InitHealthBar
  (bind _aswbp_enemy_health_bar (Utilities|Casting|CastToWBP_EnemyHealthBar (UserInterface|GetWidget (Variables|Default|GetW_HealthBar))))
  (Variables|Default|SetAs%20WBP%20Enemy%20Health%20Bar _aswbp_enemy_health_bar))

(fn UpdateHealthBar
  (bind _as_wbp_enemy_health_bar (Variables|Default|GetAs%20WBP%20Enemy%20Health%20Bar))
  (bind _w_healthbar (Variables|Default|GetW_HealthBar))
  ;[0.15 0.15 0.15 0.5] Set Percentage
  (Progress|SetPercent (Variables|/Game/GameAssets/Blueprints/Enemies/UI/WBP_EnemyHealthBar.WBP_EnemyHealthBar_C|GetHealthBar (Variables|Default|GetAs%20WBP%20Enemy%20Health%20Bar)) (/ (Variables|Default|GetHealth) (Variables|Default|GetMaxHealth)))
  ;[0.15 0.15 0.15 0.5] Set bar rotation
  (Transformation|SetWorldRotation _w_healthbar (Math|Rotator|FindLookatRotation (Transformation|GetWorldLocation _w_healthbar) (Transformation|GetWorldLocation (Variables|/Script/Engine.PlayerCameraManager|GetTransformComponent (Game|GetPlayerCameraManager 0)))) false false)
  ;[0.15 0.15 0.15 0.5] Set bar visibility
  (if (> (Variables|Default|GetHealth) 0)
    (if (>= (Variables|Default|GetHealth) (Variables|Default|GetMaxHealth))
      (Widget|SetVisibility _as_wbp_enemy_health_bar "Hidden")
      (else
        (Widget|SetVisibility _as_wbp_enemy_health_bar "Visible")))
    (else
      (Widget|SetVisibility (Variables|Default|GetAs%20WBP%20Enemy%20Health%20Bar) "Hidden"))))