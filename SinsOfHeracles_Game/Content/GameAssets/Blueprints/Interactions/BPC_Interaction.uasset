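; Interaction component that finds nearby interactable actors for its owner and lets the player interact with them.
; On BeginPlay it creates the WB_Interact widget and starts a looping timer that sphere-traces in place at the owner's location.
; A hit implementing BPI_Interaction is cached as HitActor and its look-at message is shown, otherwise both are cleared.
; IA_PlayerInteract calls InteractWithMessage on the cached actor; its BPC_ItemData check currently changes nothing.
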(event Custom|BeginInteraction
  (Utilities|Time|SetTimerbyEvent (delegate Custom|UpdateInteraction) 0.2 true))

(event Custom|UpdateInteraction
  (CallFunction|InteractionTrace))

(event Input|EnhancedActionEvents|EnhancedInputActionIA_PlayerInteract
  (params (ActionValue :type Boolean) (ElapsedSeconds :type Float%20%28double-precision%29) (TriggeredSeconds :type Float%20%28double-precision%29) (InputAction :type Input%20Action%20Object%20Reference :default "/Game/GameAssets/Blueprints/Inputs/IA_PlayerInteract.IA_PlayerInteract"))
  (:Started
    (bind _hit_actor (Variables|Default|GetHit%20Actor)
      (:then
        (Utilities|IsValid (Actor|GetComponentbyClass _hit_actor "/Game/GameAssets/Blueprints/Inventory/ItemData/BPC_ItemData.BPC_ItemData_C")
          (:Is%20Valid
            _)
          (:Is%20Not%20Valid
            _))
        (Class|BPIInteraction|Interactwith(Message) (Variables|Default|GetHit%20Actor)))
      (:else))))

(event EventBeginPlay
  (CallFunction|CreateInteractionUI)
  (CallFunction|BeginInteraction))

(fn CreateInteractionUI
  (bind _returnvalue (UserInterface|CreateWidget "/Game/GameAssets/Blueprints/Player/UI/Interactions/WB_Interact.WB_Interact_C"))
  (bind _output_get (Variables|Default|SetInteractionUI _returnvalue))
  (UserInterface|Viewport|AddtoViewport _output_get 0))

(fn InteractionTrace
  (bind _returnvalue (Components|GetOwner))
  (bind _returnvalue_2 (Transformation|GetActorLocation _returnvalue))
  (bind (_outhit _returnvalue_3) (Collision|SphereTraceByChannel _returnvalue_2 _returnvalue_2 1e+02 "TraceTypeQuery3" false 0 "None"))
  (if _returnvalue_3
    (if (Utilities|DoesObjectImplementInterface (.HitActor (Collision|BreakHitResult _outhit)) "/Game/GameAssets/Blueprints/Interactions/BPI_Interaction.BPI_Interaction_C")
      (bind _output_get (Variables|Default|SetHit%20Actor (.HitActor (Collision|BreakHitResult _outhit))))
      (bind _message (Class|BPIInteraction|Lookat(Message) _output_get))
      (Default|SetMessage (Variables|Default|GetInteractionUI) _message)
      (else
        (Variables|Default|SetHit%20Actor 0)
        (Default|SetMessage (Variables|Default|GetInteractionUI))))
    (else
      (Variables|Default|SetHit%20Actor 0)
      (Default|SetMessage (Variables|Default|GetInteractionUI)))))