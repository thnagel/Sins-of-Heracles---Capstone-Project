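; BP_King is the interactable NPC King Eurystheus, who opens a dialogue display when the player interacts with him.
; The interact event hands off to the BPCDialogue component, while LookAt returns his display name.
; When the player character leaves the sphere collision, the dialogue ends and the mouse is hidden.
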(event OnComponentEndOverlap(SphereCollision)
  (params (OverlappedComponent :type Primitive%20Component%20Object%20Reference) (OtherActor :type Actor%20Object%20Reference) (OtherComp :type Primitive%20Component%20Object%20Reference) (OtherBodyIndex :type Integer))
  (if (== OtherActor (Game|GetPlayerCharacter 0))
    (Default|EndDialogue (Variables|Default|GetBPC_Dialogue))
    (CallFunction|HideMouse)))

(event EventBeginPlay)

(event Collision|EventActorBeginOverlap
  (params (OtherActor :type Actor%20Object%20Reference)))

(event EventTick
  (params (DeltaSeconds :type Float%20%28single-precision%29)))

(event EventInteractwith
  (Default|CreateDialogDisplay (Variables|Default|GetBPC_Dialogue)))

(fn ConstructionScript)

(fn Lookat
  (return "King Eurystheus"))