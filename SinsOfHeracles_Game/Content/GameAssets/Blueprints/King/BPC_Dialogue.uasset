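; Dialogue component for the King NPC that opens and closes an on-screen dialogue box when the actor is interacted with.
; Interaction creates a display widget with speaker name and portrait, or signals speaker finished on the existing one.
; It switches the King's AI controller to talking toward the interactor.
; Ending dialogue removes the widget, returns the AI to idle and hides the mouse cursor.
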(event Custom|CreateDialogDisplay
  ;[0.15 0.15 0.15 0.5] Create Dialog Display
  (Variables|Default|GetDialogueDisplay
    (:then
      (Default|CallOnSpeakerFinished (Variables|/Game/GameAssets/Blueprints/Player/UI/Dialog/WBP_DialogDisplay.WBP_DialogDisplay_C|GetWBP_DialogBox (Variables|Default|GetDialogueDisplay))))
    (:else
      (bind _returnvalue (UserInterface|CreateWidget "/Game/GameAssets/Blueprints/Player/UI/Dialog/WBP_DialogDisplay.WBP_DialogDisplay_C" 0 (Variables|Default|GetSpeaker%20Name) (Variables|Default|GetPortrait)))
      (bind _output_get (Variables|Default|SetDialogueDisplay _returnvalue))
      (UserInterface|Viewport|AddtoViewport _output_get 0)
      (bind _aicontroller (Variables|Default|GetAIController)
        (:then
          (Default|SetStateTalking _aicontroller (Variables|Default|GetInteractor)))
        (:else)))))

(event Custom|EndDialogue
  ;[0.15 0.15 0.15 0.5] End Dialogue logic
  (bind _dialoguedisplay (Variables|Default|GetDialogueDisplay)
    (:then
      (Widget|RemovefromParent _dialoguedisplay)
      (Variables|Default|SetDialogueDisplay 0)
      (bind _aicontroller (Variables|Default|GetAIController)
        (:then
          (Default|SetStateIdle _aicontroller)
          (Variables|/Script/Engine.PlayerController|SetbShowMouseCursor (Game|GetPlayerController 0) false))
        (:else)))
    (:else)))

(event EventBeginPlay
  ;[0.15 0.15 0.15 0.5] Get ref to AIC
  (bind _asaic_king (Utilities|Casting|CastToAIC_King (AI|GetAIController (Components|GetOwner))))
  (Variables|Default|SetAIController _asaic_king))

(event EventInteractwith
  (params (Interactor :type Actor%20Object%20Reference))
  ;[0.15 0.15 0.15 0.5] Interact
  (Variables|Default|SetInteractor Interactor)
  (CallFunction|CreateDialogDisplay))

(fn Lookat
  (return ""))