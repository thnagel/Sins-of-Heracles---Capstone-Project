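; Spike trap that extends its spikes shortly after any actor overlaps its box collision and damages valid victims.
; After the delay it sets SpikesOut and sends ResolveAttackMessage to the triggering actor if that is the player or tagged Targetable, without rechecking overlap.
; A DoOnce blocks retriggering until a second delay retracts the spikes and resets it.
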(event OnComponentBeginOverlap(BoxCollision)
  (params (OverlappedComponent :type Primitive%20Component%20Object%20Reference) (OtherActor :type Actor%20Object%20Reference) (OtherComp :type Primitive%20Component%20Object%20Reference) (OtherBodyIndex :type Integer) (bFromSweep :type Boolean) (SweepResult :type Hit%20Result%20Structure%20%28by%20ref%29))
  (bind _returnvalue (Transformation|GetActorLocation OtherActor))
  (Utilities|FlowControl|DoOnce false :!label _label
    (:Completed
      (Utilities|FlowControl|Delay 0.4)
      (Variables|Default|SetSpikesOut true)
      (if (or (== OtherActor (Game|GetPlayerCharacter 0)) (Actor|ActorHasTag OtherActor "Targetable"))
        (Class|BPICombatant|ResolveAttack(Message) OtherActor self (Math|Vector|MakeVector (.x _returnvalue) (.y _returnvalue) (+ (.z _returnvalue) 5e+01)) 50)
        (Utilities|FlowControl|Delay 3.0)
        (Variables|Default|SetSpikesOut false)
        (goto _label Reset)
        (else
          (Utilities|FlowControl|Delay 3.0)
          (Variables|Default|SetSpikesOut false)
          (goto _label Reset))))))

(fn ConstructionScript)