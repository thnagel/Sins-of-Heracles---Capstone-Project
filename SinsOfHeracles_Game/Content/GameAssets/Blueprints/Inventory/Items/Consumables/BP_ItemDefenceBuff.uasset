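; BP_ItemDefenceBuff is a consumable inventory item that temporarily raises the player's Defense.
; Use casts player 0's character to BP_Player, adds a flat bonus to Defense and attaches a Niagara effect to the HeraclesMesh spine.
; A timer calls RemoveBuff after 30 seconds, matching the item's lifespan.
; RemoveBuff sets Defense to zero rather than subtracting the bonus.
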(event Custom|RemoveBuff
  (Variables|/Game/GameAssets/Blueprints/Player/BP_Player.BP_Player_C|SetDefense (Variables|Default|GetAs%20BP%20Player_0) 0))

(event EventBeginPlay
  (|CallParentFunction) ; This node is disabled and will not be called.\nDrag off pins to build functionality.
)

(event Collision|EventActorBeginOverlap
  (params (OtherActor :type Actor%20Object%20Reference))
  (|CallParentFunction OtherActor) ; This node is disabled and will not be called.\nDrag off pins to build functionality.
)

(event EventTick
  (params (DeltaSeconds :type Float%20%28single-precision%29))
  (|CallParentFunction DeltaSeconds) ; This node is disabled and will not be called.\nDrag off pins to build functionality.
)

(event EventUse
  (Actor|SetLifeSpan 3e+01)
  (bind _asbp_player (Utilities|Casting|CastToBP_Player (Game|GetPlayerCharacter 0)))
  (Variables|Default|SetAs%20BP%20Player_0 _asbp_player)
  (Variables|/Game/GameAssets/Blueprints/Player/BP_Player.BP_Player_C|SetDefense _asbp_player (+ (Variables|/Game/GameAssets/Blueprints/Player/BP_Player.BP_Player_C|GetDefense _asbp_player) 10))
  (Niagara|SpawnSystemAttached "/Game/GameAssets/Assets/Potions/NS_DefenceBuff.NS_DefenceBuff" (Variables|/Game/GameAssets/Blueprints/Player/BP_Player.BP_Player_C|GetHeraclesMesh (Variables|Default|GetAs%20BP%20Player_0)) "spine_3" "0.000000,0.000000,90.000000" "0, 0, 0" "KeepRelativeOffset" true)
  (Utilities|Time|SetTimerbyEvent (delegate Custom|RemoveBuff) 3e+01 false true))

(fn ConstructionScript
  (|CallParentFunction))