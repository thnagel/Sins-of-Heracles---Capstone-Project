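; BP_ItemDamageBuff is a consumable inventory item that temporarily boosts the player's damage.
; Use adds a flat bonus to both melee and ranged attack damage on BP_Player and attaches a Niagara effect to the character's mesh.
; A timer calls RemoveBuff to subtract the same bonus, with the item actor's lifespan set to the same duration as that timer.
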(event Custom|RemoveBuff
  (bind _as_bp_player_0 (Variables|Default|GetAs%20BP%20Player_0))
  (bind _as_bp_player_0_2 (Variables|Default|GetAs%20BP%20Player_0))
  (Variables|/Game/GameAssets/Blueprints/Player/BP_Player.BP_Player_C|SetRanged%20Attack%20Damage _as_bp_player_0 (- (Variables|/Game/GameAssets/Blueprints/Player/BP_Player.BP_Player_C|GetRanged%20Attack%20Damage _as_bp_player_0) 20))
  (Variables|/Game/GameAssets/Blueprints/Player/BP_Player.BP_Player_C|SetAttack%20Damage _as_bp_player_0_2 (- (Variables|/Game/GameAssets/Blueprints/Player/BP_Player.BP_Player_C|GetAttack%20Damage _as_bp_player_0_2) 20)))

(event EventBeginPlay
  (|CallParentFunction) ; This node is disabled and will not be called.\nDrag off pins to build functionality.
)

(event Collision|EventActorBeginOverlap
  (params (OtherActor :type Actor%20Object%20Reference))
  (|CallParentFunction OtherActor) ; This node is disabled and will not be called.\nDrag off pins to build functionality.
)

(event EventTick
  (params (DeltaSeconds :type Float%20%28single-precision%29))
  (|CallParentFunction DeltaSeconds) ; This node is disabled and will not be called.\nDrag off pins to build functionality.
)

(event EventUse
  (Actor|SetLifeSpan 3e+01)
  (bind _asbp_player (Utilities|Casting|CastToBP_Player (Game|GetPlayerCharacter 0)))
  (Variables|Default|SetAs%20BP%20Player_0 _asbp_player)
  (Variables|/Game/GameAssets/Blueprints/Player/BP_Player.BP_Player_C|SetRanged%20Attack%20Damage _asbp_player (+ (Variables|/Game/GameAssets/Blueprints/Player/BP_Player.BP_Player_C|GetRanged%20Attack%20Damage _asbp_player) 20))
  (Variables|/Game/GameAssets/Blueprints/Player/BP_Player.BP_Player_C|SetAttack%20Damage _asbp_player (+ (Variables|/Game/GameAssets/Blueprints/Player/BP_Player.BP_Player_C|GetAttack%20Damage _asbp_player) 20))
  (Niagara|SpawnSystemAttached "/Game/GameAssets/Assets/Potions/NS_DamageBuff.NS_DamageBuff" (Variables|/Game/GameAssets/Blueprints/Player/BP_Player.BP_Player_C|GetHeraclesMesh (Variables|Default|GetAs%20BP%20Player_0)) "spine_3" "0.000000,0.000000,100.000000" "0, 0, 0" "KeepRelativeOffset" true)
  (Utilities|Time|SetTimerbyEvent (delegate Custom|RemoveBuff) 3e+01 false true))

(fn ConstructionScript
  (|CallParentFunction))