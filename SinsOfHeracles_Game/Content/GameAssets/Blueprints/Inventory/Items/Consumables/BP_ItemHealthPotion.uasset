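; BP_ItemHealthPotion is a consumable inventory item that restores a fixed amount of the player's health.
; Its Use event casts player character 0 to BP_Player and adds the heal directly to Health, capping the result at MaxHealth.
; The graph contains no other active gameplay logic and does not handle removing or consuming the item.
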(event EventBeginPlay
  (|CallParentFunction) ; This node is disabled and will not be called.\nDrag off pins to build functionality.
)

(event Collision|EventActorBeginOverlap
  (params (OtherActor :type Actor%20Object%20Reference))
  (|CallParentFunction OtherActor) ; This node is disabled and will not be called.\nDrag off pins to build functionality.
)

(event EventTick
  (params (DeltaSeconds :type Float%20%28single-precision%29))
  (|CallParentFunction DeltaSeconds) ; This node is disabled and will not be called.\nDrag off pins to build functionality.
)

(event EventUse
  (bind _asbp_player (Utilities|Casting|CastToBP_Player (Game|GetPlayerCharacter 0)))
  (if (> (+ (Variables|/Game/GameAssets/Blueprints/Player/BP_Player.BP_Player_C|GetHealth _asbp_player) 25) (Variables|/Game/GameAssets/Blueprints/Player/BP_Player.BP_Player_C|GetMaxHealth _asbp_player))
    (Variables|/Game/GameAssets/Blueprints/Player/BP_Player.BP_Player_C|SetHealth _asbp_player (Variables|/Game/GameAssets/Blueprints/Player/BP_Player.BP_Player_C|GetMaxHealth _asbp_player))
    (else
      (Variables|/Game/GameAssets/Blueprints/Player/BP_Player.BP_Player_C|SetHealth _asbp_player (+ (Variables|/Game/GameAssets/Blueprints/Player/BP_Player.BP_Player_C|GetHealth _asbp_player) 25)))))

(fn ConstructionScript
  (|CallParentFunction))