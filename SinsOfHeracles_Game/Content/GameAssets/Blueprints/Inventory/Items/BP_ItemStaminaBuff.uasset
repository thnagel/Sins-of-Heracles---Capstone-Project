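; Inventory item that grants the player a temporary max stamina buff when used.
; Use finds BP_Player, saves its max stamina, multiplies max and current stamina by StaminaIncrease, then starts a timer.
; Repeat uses while active skip the boost and only set the timer again, so the buff does not stack on that item instance.
; BuffTimer clears the effect, restoring max stamina and rescaling current stamina proportionally.
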(event Custom|BuffTimer
  (bind _basestamina (Variables|Default|GetBaseStamina))
  (Variables|Default|SetIsInEffect? false)
  (bind _returnvalue (Actor|GetActorOfClass "/Game/GameAssets/Blueprints/Player/BP_Player.BP_Player_C"))
  (Variables|/Game/GameAssets/Blueprints/Player/BP_Player.BP_Player_C|SetStamina _returnvalue (/ (* (Variables|/Game/GameAssets/Blueprints/Player/BP_Player.BP_Player_C|GetStamina _returnvalue) _basestamina) (Variables|/Game/GameAssets/Blueprints/Player/BP_Player.BP_Player_C|GetMaxStamina _returnvalue)))
  (Variables|/Game/GameAssets/Blueprints/Player/BP_Player.BP_Player_C|SetMaxStamina _returnvalue _basestamina))

(event EventBeginPlay
  (|CallParentFunction) ; This node is disabled and will not be called.\nDrag off pins to build functionality.
)

(event Collision|EventActorBeginOverlap
  (params (OtherActor :type Actor%20Object%20Reference))
  (|CallParentFunction OtherActor) ; This node is disabled and will not be called.\nDrag off pins to build functionality.
)

(event EventTick
  (params (DeltaSeconds :type Float%20%28single-precision%29))
  (|CallParentFunction DeltaSeconds) ; This node is disabled and will not be called.\nDrag off pins to build functionality.
)

(fn ConstructionScript
  (|CallParentFunction))

(fn Use
  (bind _returnvalue (Actor|GetActorOfClass "/Game/GameAssets/Blueprints/Player/BP_Player.BP_Player_C"))
  (if (Variables|Default|GetIsInEffect?)
    _
    (else
      (bind _output_get (Variables|Default|SetBaseStamina (Variables|/Game/GameAssets/Blueprints/Player/BP_Player.BP_Player_C|GetMaxStamina _returnvalue)))
      (Variables|/Game/GameAssets/Blueprints/Player/BP_Player.BP_Player_C|SetMaxStamina _returnvalue (* _output_get (Variables|Default|GetStaminaIncrease)))
      (Variables|/Game/GameAssets/Blueprints/Player/BP_Player.BP_Player_C|SetStamina _returnvalue (Math|Float|Truncate (* (Variables|/Game/GameAssets/Blueprints/Player/BP_Player.BP_Player_C|GetStamina _returnvalue) (Variables|Default|GetStaminaIncrease))))
      (Variables|Default|SetIsInEffect? true)))
  (Utilities|Time|SetTimerbyEvent (EventDispatchers|CreateEvent :!event Custom|BuffTimer) (Variables|Default|GetTime))
  (|CallParentFunction))