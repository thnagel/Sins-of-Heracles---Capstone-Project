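; World pickup actor for leather gauntlets that the player can take into their inventory.
; GetItemDetails searches the item, consumable, weapon and armour data tables in turn, supplying the item type and look-at prompt name.
; Interacting adds the stack to the inventory; a full pickup logs a HUD banner and destroys the actor, otherwise the leftover quantity remains.
; The first sufficiently fast mesh hit plays a pitch-randomised glass drop sound.
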(event OnComponentHit(StaticMesh)
  (params (HitComponent :type Primitive%20Component%20Object%20Reference) (OtherActor :type Actor%20Object%20Reference) (OtherComp :type Primitive%20Component%20Object%20Reference) (NormalImpulse :type Vector :default "0, 0, 0") (Hit :type Hit%20Result%20Structure%20%28by%20ref%29))
  (if (not (Variables|Default|GetHasPlayedSFX))
    (if (> (Math|Vector|VectorLength (Transformation|GetComponentVelocity (Variables|Default|GetStaticMesh))) 1e+02)
      (Audio|PlaySoundatLocation "/Game/GameAssets/Assets/SFX/Items/GlassItemDrop.GlassItemDrop" (.ImpactPoint (Collision|BreakHitResult Hit)) "0, 0, 0" 0.2 (Math|Random|RandomFloatinRange 0.9 1.1) 0.0 0 0 0 0)
      (Variables|Default|SetHasPlayedSFX true))))

(event EventBeginPlay)

(event Collision|EventActorBeginOverlap
  (params (OtherActor :type Actor%20Object%20Reference)))

(event EventTick
  (params (DeltaSeconds :type Float%20%28single-precision%29)))

(event EventInteractwith
  (params (Interactor :type Actor%20Object%20Reference))
  (bind _bpc_itemdata (Variables|Default|GetBPC_ItemData))
  (bind _item (Variables|/Game/GameAssets/Blueprints/Inventory/ItemData/BPC_ItemData.BPC_ItemData_C|GetItem _bpc_itemdata))
  (bind (_datatable _rowname) (Utilities|Struct|BreakDataTableRowHandle _item))
  (bind _playerinventory (CallFunction|GetPlayerInventory))
  (bind (_itemquantityleft _notfull) (Default|AddtoInventory _playerinventory _rowname (Variables|/Game/GameAssets/Blueprints/Inventory/ItemData/BPC_ItemData.BPC_ItemData_C|GetItemQuantity _bpc_itemdata) (Utilities|ResolveSoftReference _datatable) (.ItemType (CallFunction|GetItemDetails)) false))
  ;[0.15 0.15 0.15 0.5] Handle Hud notification
  (if (and _notfull (== _itemquantityleft 0))
    (bind _asbp_player (Utilities|Casting|CastToBP_Player (Game|GetPlayerCharacter 0)))
    (Variables|Default|SetAs%20BP%20Player _asbp_player)
    (Default|AddNewBanner (Variables|/Game/GameAssets/Blueprints/Player/UI/HUD/WBP_HUD.WBP_HUD_C|GetWBP_PickUpLog (Variables|/Game/GameAssets/Blueprints/Player/BP_Player.BP_Player_C|GetWBP_HUD (Variables|Default|GetAs%20BP%20Player))) _rowname (stale _output_get))
    (Actor|DestroyActor)
    (else
      (bind _output_get (Variables|/Game/GameAssets/Blueprints/Inventory/ItemData/BPC_ItemData.BPC_ItemData_C|SetItemQuantity (Variables|Default|GetBPC_ItemData) _itemquantityleft)))))

(fn ConstructionScript)

(fn GetItemDetails
  (bind _bpc_itemdata (Variables|Default|GetBPC_ItemData))
  (bind _item (Variables|/Game/GameAssets/Blueprints/Inventory/ItemData/BPC_ItemData.BPC_ItemData_C|GetItem _bpc_itemdata))
  (bind _rowname (Utilities|Struct|BreakDataTableRowHandle _item))
  (bind _returnvalue (Utilities|GetDataTableRow "/Game/GameAssets/Blueprints/Inventory/ItemData/DataTables/DT_ItemData.DT_ItemData" _rowname)
    (:then
      (return (.itemname _returnvalue) (.itemicon _returnvalue) (.itemvalue _returnvalue) (.itemstacksize _returnvalue) (.sound _returnvalue) (.description _returnvalue) "NewEnumerator0"))
    (:RowNotFound
      (bind _returnvalue_2 (Utilities|GetDataTableRow "/Game/GameAssets/Blueprints/Inventory/ItemData/DataTables/DT_Consumables.DT_Consumables" _rowname)
        (:then
          (return (.itemname _returnvalue_2) (.itemicon _returnvalue_2) (.itemvalue _returnvalue_2) (.itemstacksize _returnvalue_2) (.sound _returnvalue_2) (.description _returnvalue_2) "NewEnumerator1"))
        (:RowNotFound
          (bind _returnvalue_3 (Utilities|GetDataTableRow "/Game/GameAssets/Blueprints/Inventory/ItemData/DataTables/DT_Weapons.DT_Weapons" _rowname)
            (:then
              (return (.itemname _returnvalue_3) (.itemicon _returnvalue_3) (.itemvalue _returnvalue_3) (.itemstacksize _returnvalue_3) (.sound _returnvalue_3) (.description _returnvalue_3) "NewEnumerator2"))
            (:RowNotFound
              (bind _returnvalue_4 (Utilities|GetDataTableRow "/Game/GameAssets/Blueprints/Inventory/ItemData/DataTables/DT_Armours.DT_Armours" _rowname)
                (:then
                  (return (.itemname _returnvalue_4) (.itemicon _returnvalue_4) (.itemvalue _returnvalue_4) (.itemstacksize _returnvalue_4) (.sound _returnvalue_4) (.description _returnvalue_4) "NewEnumerator3"))))))))))

(fn Lookat
  (return (Utilities|Text|FormatText "Take {Name} [{Quantity}]" (.ItemName (CallFunction|GetItemDetails)) (Variables|/Game/GameAssets/Blueprints/Inventory/ItemData/BPC_ItemData.BPC_ItemData_C|GetItemQuantity (Variables|Default|GetBPC_ItemData)))))