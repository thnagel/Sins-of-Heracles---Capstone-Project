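; BP_ItemDefenseBuff is an inventory item that temporarily boosts the player's maximum health as a defense buff.
; Use stores the base MaxHealth, multiplies MaxHealth and current Health by HpIncrease, then starts a timer and calls the parent Use.
; An IsInEffect flag prevents stacking, while repeated use still sets the timer again.
; BuffTimer clears the flag, scales Health back proportionally and restores the base MaxHealth.
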(event Custom|BuffTimer
  (bind _basehp (Variables|Default|GetBaseHp))
  (Variables|Default|SetIsInEffect? false)
  (bind _returnvalue (Actor|GetActorOfClass "/Game/GameAssets/Blueprints/Player/BP_Player.BP_Player_C"))
  (Variables|/Game/GameAssets/Blueprints/Player/BP_Player.BP_Player_C|SetHealth _returnvalue (/ (* (Variables|/Game/GameAssets/Blueprints/Player/BP_Player.BP_Player_C|GetHealth _returnvalue) _basehp) (Variables|/Game/GameAssets/Blueprints/Player/BP_Player.BP_Player_C|GetMaxHealth _returnvalue)))
  (Variables|/Game/GameAssets/Blueprints/Player/BP_Player.BP_Player_C|SetMaxHealth _returnvalue _basehp))

(event EventBeginPlay
  (|CallParentFunction) ; This node is disabled and will not be called.\nDrag off pins to build functionality.
)

(event Collision|EventActorBeginOverlap
  (params (OtherActor :type Actor%20Object%20Reference))
  (|CallParentFunction OtherActor) ; This node is disabled and will not be called.\nDrag off pins to build functionality.
)

(event EventTick
  (params (DeltaSeconds :type Float%20%28single-precision%29))
  (|CallParentFunction DeltaSeconds) ; This node is disabled and will not be called.\nDrag off pins to build functionality.
)

(fn ConstructionScript
  (|CallParentFunction))

(fn Use
  (bind _returnvalue (Actor|GetActorOfClass "/Game/GameAssets/Blueprints/Player/BP_Player.BP_Player_C"))
  (if (Variables|Default|GetIsInEffect?)
    _
    (else
      (bind _output_get (Variables|Default|SetBaseHp (Variables|/Game/GameAssets/Blueprints/Player/BP_Player.BP_Player_C|GetMaxHealth _returnvalue)))
      (Variables|/Game/GameAssets/Blueprints/Player/BP_Player.BP_Player_C|SetMaxHealth _returnvalue (* _output_get (Variables|Default|GetHpIncrease)))
      (Variables|/Game/GameAssets/Blueprints/Player/BP_Player.BP_Player_C|SetHealth _returnvalue (Math|Float|Truncate (* (Variables|/Game/GameAssets/Blueprints/Player/BP_Player.BP_Player_C|GetHealth _returnvalue) (Variables|Default|GetHpIncrease))))
      (Variables|Default|SetIsInEffect? true)))
  (Utilities|Time|SetTimerbyEvent (EventDispatchers|CreateEvent :!event Custom|BuffTimer) (Variables|Default|GetTime))
  (|CallParentFunction))