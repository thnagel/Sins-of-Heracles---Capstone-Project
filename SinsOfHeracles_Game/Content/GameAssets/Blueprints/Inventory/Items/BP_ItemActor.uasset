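; BP_ItemActor is a world inventory item with item data and a static mesh.
; It looks up its row from the data table referenced by its BPCItemData component and formats a "Take Name [Quantity]" look-at prompt from it.
; A mesh hit above a speed threshold plays a glass drop sound with randomized pitch, limited to once by a flag.
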(event OnComponentHit(StaticMesh)
  (params (HitComponent :type Primitive%20Component%20Object%20Reference) (OtherActor :type Actor%20Object%20Reference) (OtherComp :type Primitive%20Component%20Object%20Reference) (NormalImpulse :type Vector :default "0, 0, 0") (Hit :type Hit%20Result%20Structure%20%28by%20ref%29))
  (if (not (Variables|Default|GetHasPlayedSFX))
    (if (> (Math|Vector|VectorLength (Transformation|GetComponentVelocity (Variables|Default|GetStaticMesh))) 1e+02)
      (Audio|PlaySoundatLocation "/Game/GameAssets/Assets/SFX/Items/GlassItemDrop.GlassItemDrop" (.ImpactPoint (Collision|BreakHitResult Hit)) "0, 0, 0" 0.2 (Math|Random|RandomFloatinRange 0.9 1.1) 0.0 0 0 0 0)
      (Variables|Default|SetHasPlayedSFX true))))

(event EventBeginPlay)

(event Collision|EventActorBeginOverlap
  (params (OtherActor :type Actor%20Object%20Reference)))

(event EventTick
  (params (DeltaSeconds :type Float%20%28single-precision%29)))

(fn ConstructionScript)

(fn GetItemDetails
  (bind _bpc_itemdata (Variables|Default|GetBPC_ItemData))
  (bind _item (Variables|/Game/GameAssets/Blueprints/Inventory/ItemData/BPC_ItemData.BPC_ItemData_C|GetItem _bpc_itemdata))
  (bind (_datatable _rowname) (Utilities|Struct|BreakDataTableRowHandle _item))
  (bind _returnvalue (Utilities|GetDataTableRow _datatable _rowname)
    (:then
      (return _returnvalue))))

(fn Lookat
  (return (Utilities|Text|FormatText "Take {Name} [{Quantity}]" (.ItemName (Utilities|Struct|BreakS_ItemDetails (CallFunction|GetItemDetails))) (Variables|/Game/GameAssets/Blueprints/Inventory/ItemData/BPC_ItemData.BPC_ItemData_C|GetItemQuantity (Variables|Default|GetBPC_ItemData)))))