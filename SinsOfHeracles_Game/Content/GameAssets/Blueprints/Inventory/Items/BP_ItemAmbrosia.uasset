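; BP_ItemAmbrosia is a healing inventory item that restores the player's health when used.
; Its Use override finds the BP_Player via GetActorOfClass and adds HealAmmount to Health, clamped between zero and MaxHealth.
; It then calls the parent Use; the event graph holds only disabled stub events.
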(event EventBeginPlay
  (|CallParentFunction) ; This node is disabled and will not be called.\nDrag off pins to build functionality.
)

(event Collision|EventActorBeginOverlap
  (params (OtherActor :type Actor%20Object%20Reference))
  (|CallParentFunction OtherActor) ; This node is disabled and will not be called.\nDrag off pins to build functionality.
)

(event EventTick
  (params (DeltaSeconds :type Float%20%28single-precision%29))
  (|CallParentFunction DeltaSeconds) ; This node is disabled and will not be called.\nDrag off pins to build functionality.
)

(fn ConstructionScript
  (|CallParentFunction))

(fn Use
  (bind _returnvalue (Actor|GetActorOfClass "/Game/GameAssets/Blueprints/Player/BP_Player.BP_Player_C"))
  (Variables|/Game/GameAssets/Blueprints/Player/BP_Player.BP_Player_C|SetHealth _returnvalue (Math|Integer|Clamp(Integer) (+ (Variables|/Game/GameAssets/Blueprints/Player/BP_Player.BP_Player_C|GetHealth _returnvalue) (Variables|Default|GetHealAmmount)) 0 (Variables|/Game/GameAssets/Blueprints/Player/BP_Player.BP_Player_C|GetMaxHealth _returnvalue)))
  (|CallParentFunction))