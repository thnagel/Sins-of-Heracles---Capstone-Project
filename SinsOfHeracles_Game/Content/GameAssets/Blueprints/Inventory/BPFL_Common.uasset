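; Blueprint function library of common player helpers for the inventory system.
; GetPlayerInventory returns the inventory component on player 0's character when it is valid.
; ShowMouse displays the cursor and switches to game-and-UI input focused on a given widget.
; HideMouse hides the cursor and restores game-only input, after checking that the player controller is valid.
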(fn GetPlayerInventory
  (bind _returnvalue (Game|GetPlayerCharacter 0))
  (bind _returnvalue_2 (Actor|GetComponentbyClass _returnvalue "/Game/GameAssets/Blueprints/Inventory/BPC_Inventory.BPC_Inventory_C"))
  (Utilities|IsValid _returnvalue_2
    (:Is%20Valid
      (return _returnvalue_2))))

(fn ShowMouse
  (params (InWidgetToFocus :type Widget%20Object%20Reference))
  (bind _returnvalue (Game|GetPlayerController 0))
  (Variables|/Script/Engine.PlayerController|SetbShowMouseCursor _returnvalue true)
  (Input|SetInputModeGameandUI _returnvalue InWidgetToFocus "DoNotLock" true false))

(fn HideMouse
  (bind _returnvalue (Game|GetPlayerController 0))
  (Utilities|IsValid _returnvalue
    (:Is%20Valid
      (Variables|/Script/Engine.PlayerController|SetbShowMouseCursor _returnvalue false)
      (Input|SetInputModeGameOnly _returnvalue false))))