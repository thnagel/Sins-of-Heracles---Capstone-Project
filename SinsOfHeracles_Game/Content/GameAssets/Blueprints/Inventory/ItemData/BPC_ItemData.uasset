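; Item data component for pickup actors that adds its item to the player's inventory on interact.
; A full pickup posts a banner to the HUD pickup log and destroys the owner; otherwise the leftover quantity stays on the component.
; GetItemDetails searches the item, consumable, weapon and armour data tables in turn by row name, assigning a fixed item type for the latter three.
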(event EventBeginPlay
  ;[0.15 0.15 0.15 0.5] Get BP_Player reference
  (bind _asbp_player (Utilities|Casting|CastToBP_Player (Game|GetPlayerCharacter 0)))
  (Variables|Default|SetAs%20BP%20Player _asbp_player))

(event EventInteractwith
  (params (Interactor :type Actor%20Object%20Reference))
  (bind _item (Variables|Default|GetItem))
  (bind (_datatable _rowname) (Utilities|Struct|BreakDataTableRowHandle _item))
  (bind _playerinventory (CallFunction|GetPlayerInventory))
  (bind (_itemquantityleft _notfull) (Default|AddtoInventory _playerinventory _rowname (Variables|Default|GetItemQuantity) (Utilities|ResolveSoftReference _datatable) (.Out%20Row%20Item%20Type (CallFunction|GetItemDetails))))
  (if (and _notfull (== _itemquantityleft 0))
    ;[0.15 0.15 0.15 0.5] Update HUD
    (Default|AddNewBanner (Variables|/Game/GameAssets/Blueprints/Player/UI/HUD/WBP_HUD.WBP_HUD_C|GetWBP_PickUpLog (Variables|/Game/GameAssets/Blueprints/Player/BP_Player.BP_Player_C|GetWBP_HUD (Variables|Default|GetAs%20BP%20Player))) _rowname (stale _output_get))
    (Actor|DestroyActor (Components|GetOwner))
    (else
      (bind _output_get (Variables|Default|SetItemQuantity _itemquantityleft)))))

(fn GetItemDetails
  (bind _item (Variables|Default|GetItem))
  (bind _rowname (Utilities|Struct|BreakDataTableRowHandle _item))
  (bind _returnvalue (Utilities|GetDataTableRow "/Game/GameAssets/Blueprints/Inventory/ItemData/DataTables/DT_ItemData.DT_ItemData" _rowname)
    (:then
      (return (.itemname _returnvalue) (.itemicon _returnvalue) (.itemvalue _returnvalue) (.itemstacksize _returnvalue) (.sound _returnvalue) (.description _returnvalue) (.itemtype _returnvalue)))
    (:RowNotFound
      (bind _returnvalue_2 (Utilities|GetDataTableRow "/Game/GameAssets/Blueprints/Inventory/ItemData/DataTables/DT_Consumables.DT_Consumables" _rowname)
        (:then
          (return (.itemname _returnvalue_2) (.itemicon _returnvalue_2) (.itemvalue _returnvalue_2) (.itemstacksize _returnvalue_2) (.sound _returnvalue_2) (.description _returnvalue_2) "NewEnumerator1"))
        (:RowNotFound
          (bind _returnvalue_3 (Utilities|GetDataTableRow "/Game/GameAssets/Blueprints/Inventory/ItemData/DataTables/DT_Weapons.DT_Weapons" _rowname)
            (:then
              (return (.itemname _returnvalue_3) (.itemicon _returnvalue_3) (.itemvalue _returnvalue_3) (.itemstacksize _returnvalue_3) (.sound _returnvalue_3) (.description _returnvalue_3) "NewEnumerator2"))
            (:RowNotFound
              (bind _returnvalue_4 (Utilities|GetDataTableRow "/Game/GameAssets/Blueprints/Inventory/ItemData/DataTables/DT_Armours.DT_Armours" _rowname)
                (:then
                  (return (.itemname _returnvalue_4) (.itemicon _returnvalue_4) (.itemvalue _returnvalue_4) (.itemstacksize _returnvalue_4) (.sound _returnvalue_4) (.description _returnvalue_4) "NewEnumerator3"))))))))))

(fn Lookat
  (return ""))