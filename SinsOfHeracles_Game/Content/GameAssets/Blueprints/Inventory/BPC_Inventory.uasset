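; Inventory component that stores stackable items in a fixed number of slots, toggles the player inventory widget and plays item sounds.
; Adding fills matching stacks before empty slots, using stack sizes from DT_ItemData.
; Slots support splitting, merging or swapping across inventories and bulk return, with updates recounting Ichor currency for the player's HUD.
; It also totals item value and generates random contents from a filtered item table, optionally seeded with Ichor.
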(event Custom|UpdateInventory
  ;[0.15 0.15 0.15 0.5] Update the inventory and set the correct total value
  (Default|CallOnInventoryUpdated)
  (bind _totalcurrency (CallFunction|GetTotalCurrency))
  (Variables|Default|SetIchorAmount _totalcurrency)
  ;[0.15 0.15 0.15 0.5] Update HUD
  (Default|SetIchorNumber (Variables|/Game/GameAssets/Blueprints/Player/UI/WBP_HUD.WBP_HUD_C|GetWBP_Ichor (Variables|/Game/GameAssets/Blueprints/Player/BP_Player.BP_Player_C|GetWBP_HUD (Variables|Default|GetAs%20BP%20Player)))))

(event Input|EnhancedActionEvents|EnhancedInputActionIA_Inventory
  (params (ActionValue :type Boolean) (ElapsedSeconds :type Float%20%28double-precision%29) (TriggeredSeconds :type Float%20%28double-precision%29) (InputAction :type Input%20Action%20Object%20Reference :default "/Game/GameAssets/Blueprints/Inputs/IA_Inventory.IA_Inventory"))
  ;[0.15 0.15 0.15 0.5] Open/Close inventory with assigned key
  (:Started
    (CallFunction|ToggleInventory)))

(event EventBeginPlay
  ;[0.15 0.15 0.15 0.5] Set the default size of inventories to 24
  (Utilities|Array|Resize (Variables|Default|GetInventorySlots) (Variables|Default|GetInventorySize))
  ;[0.15 0.15 0.15 0.5] Get BP_Player reference
  (bind _asbp_player (Utilities|Casting|CastToBP_Player (Game|GetPlayerCharacter 0)))
  (Variables|Default|SetAs%20BP%20Player _asbp_player))

(event Input|KeyboardEvents|DebugKey0
  (params (Key :type Key%20Structure) (ActionValue :type Input%20Action%20Value%20Structure))
  ;[0.15 0.15 0.15 0.5] DEBUG Can print player inventory content with 0
  (:Pressed
    (CallFunction|Printinventory)))

(fn AddtoInventory
  (params (ItemID :type Name) (ItemQuantity :type Integer))
  (bind (_array_index _found) (CallFunction|SlotsAvailable))
  (bind _output_get (LocalVariables|SetLocalItemQuantity ItemQuantity))
  (while (and (> _output_get 0) (not (LocalVariables|GetLocalIsInventoryFull)))
    (bind (_array_index_2 _found_2) (CallFunction|FindMatchingSlot ItemID))
    (if _found_2
      (CallFunction|AddItemtoStack _array_index_2 1)
      (Math|Integer|DecrementInt (LocalVariables|GetLocalItemQuantity) :!label _label)
      (elif _found
        (CallFunction|CreateNewStack _array_index ItemID 1)
        (goto _label)
        (else
          (LocalVariables|SetLocalIsInventoryFull true)))))
  (if (== (Components|GetOwner) (Game|GetPlayerCharacter 0))
    (CallFunction|PlayItemSound ItemID)
    (CallFunction|UpdateInventory)
    (return (LocalVariables|GetLocalItemQuantity) (not (LocalVariables|GetLocalIsInventoryFull)))))

(fn Printinventory
  (for (_array_element _array_index) (Variables|Default|GetInventorySlots)
    (Development|PrintString (Utilities|String|Append (Utilities|String|ToString(Integer) _array_index) ": " (Utilities|String|ToString(Name) (.ItemID (Utilities|Struct|BreakS_InventorySlot _array_element))) " = " (Utilities|String|ToString(Integer) (.ItemQuantity (Utilities|Struct|BreakS_InventorySlot _array_element)))))))

(fn ToggleInventory
  (bind _playerinventoryui (Variables|Default|GetPlayerInventoryUI)
    (:then
      (Audio|PlaySound2D "/Game/GameAssets/Assets/SFX/Inventory/UI_Inventory_Close.UI_Inventory_Close" 0.3 1.0 0.0 0 0)
      (Widget|RemovefromParent _playerinventoryui)
      (Variables|Default|SetPlayerInventoryUI 0))
    (:else
      (Audio|PlaySound2D "/Game/GameAssets/Assets/SFX/Inventory/UI_Inventory_Open.UI_Inventory_Open" 0.4 1.0 0.0 0 0)
      (bind _returnvalue (UserInterface|CreateWidget "/Game/GameAssets/Blueprints/Player/UI/Inventory/WBP_PlayerInventory.WBP_PlayerInventory_C"))
      (bind _output_get (Variables|Default|SetPlayerInventoryUI _returnvalue))
      (UserInterface|Viewport|AddtoViewport _output_get 0))))

(fn FindMatchingSlot
  (params (ItemID :type Name))
  (for (_array_element _array_index) (Variables|Default|GetInventorySlots)
    (if (and (== (.ItemID (Utilities|Struct|BreakS_InventorySlot _array_element)) ItemID) (< (.ItemQuantity (Utilities|Struct|BreakS_InventorySlot _array_element)) (.ItemStackSize (Utilities|Struct|BreakS_ItemDetails (CallFunction|GetItemDetails ItemID)))))
      (return _array_index true)))
  (return -1 false))

(fn GetItemDetails
  (params (ItemID :type Name))
  (bind _returnvalue (Utilities|GetDataTableRow "/Game/GameAssets/Blueprints/Inventory/ItemData/DataTables/DT_ItemData.DT_ItemData" ItemID)
    (:then
      (return _returnvalue))))

(fn AddItemtoStack
  (params (Index :type Integer) (ItemQuantity :type Integer))
  (bind _inventoryslots (Variables|Default|GetInventorySlots))
  (bind _output (Utilities|Array|Get(acopy) _inventoryslots Index))
  (Utilities|Array|SetArrayElem (Variables|Default|GetInventorySlots) Index (Utilities|Struct|MakeS_InventorySlot (.itemid _output) (+ (.itemquantity _output) ItemQuantity))))

(fn SlotsAvailable
  (for (_array_element _array_index) (Variables|Default|GetInventorySlots)
    (if (== (.ItemQuantity (Utilities|Struct|BreakS_InventorySlot _array_element)) 0)
      (return _array_index true)))
  (return -1 false))

(fn CreateNewStack
  (params (Index :type Integer) (itemID :type Name) (ItemQuantity :type Integer))
  (Utilities|Array|SetArrayElem (Variables|Default|GetInventorySlots) Index (Utilities|Struct|MakeS_InventorySlot itemID ItemQuantity)))

(fn GetTotalCurrency
  (for _array_element (Variables|Default|GetInventorySlots)
    (if (== (.ItemID (Utilities|Struct|BreakS_InventorySlot _array_element)) "Ichor")
      (LocalVariables|SetLocalTotalCurrency (+ (.ItemQuantity (Utilities|Struct|BreakS_InventorySlot _array_element)) (LocalVariables|GetLocalTotalCurrency)))))
  (return (LocalVariables|GetLocalTotalCurrency)))

(fn TransferSlots
  (params (SourceInventory :type BPC%20Inventory%20Object%20Reference) (SourceIndex :type Integer) (Index :type Integer))
  (LocalVariables|SetLocalTargetItem (Utilities|Array|Get(acopy) (Variables|Default|GetInventorySlots) Index))
  (LocalVariables|SetLocalSourceItem (Utilities|Array|Get(acopy) (Variables|BPC_Inventory_C|GetInventorySlots SourceInventory) SourceIndex))
  (Utilities|FlowControl|Sequence
    (:then_0
      (if (== (.ItemID (Utilities|Struct|BreakS_InventorySlot (LocalVariables|GetLocalSourceItem))) (.ItemID (Utilities|Struct|BreakS_InventorySlot (LocalVariables|GetLocalTargetItem))))
        (bind _output_get (LocalVariables|SetLocalTotalQuantity (+ (.ItemQuantity (Utilities|Struct|BreakS_InventorySlot (LocalVariables|GetLocalSourceItem))) (.ItemQuantity (Utilities|Struct|BreakS_InventorySlot (LocalVariables|GetLocalTargetItem))))))
        (if (> (+ (.ItemQuantity (Utilities|Struct|BreakS_InventorySlot (LocalVariables|GetLocalSourceItem))) (.ItemQuantity (Utilities|Struct|BreakS_InventorySlot (LocalVariables|GetLocalTargetItem)))) (.ItemStackSize (Utilities|Struct|BreakS_ItemDetails (CallFunction|GetItemDetails (.ItemID (Utilities|Struct|BreakS_InventorySlot (LocalVariables|GetLocalTargetItem)))))))
          (LocalVariables|SetLocalQuantityLeft (- _output_get (.ItemStackSize (Utilities|Struct|BreakS_ItemDetails (CallFunction|GetItemDetails (.ItemID (Utilities|Struct|BreakS_InventorySlot (LocalVariables|GetLocalTargetItem))))))))
          (CallFunction|CreateNewStack Index (.ItemID (Utilities|Struct|BreakS_InventorySlot (LocalVariables|GetLocalTargetItem))) (.ItemStackSize (Utilities|Struct|BreakS_ItemDetails (CallFunction|GetItemDetails (.ItemID (Utilities|Struct|BreakS_InventorySlot (LocalVariables|GetLocalTargetItem)))))))
          (CallFunction|CreateNewStack SourceInventory SourceIndex (.ItemID (Utilities|Struct|BreakS_InventorySlot (LocalVariables|GetLocalTargetItem))) (LocalVariables|GetLocalQuantityLeft))
          (else
            (CallFunction|CreateNewStack Index (.itemid (LocalVariables|GetLocalTargetItem)) (LocalVariables|GetLocalTotalQuantity))
            (CallFunction|CreateNewStack SourceInventory SourceIndex "None")))
        (else
          (CallFunction|CreateNewStack Index (.itemid (LocalVariables|GetLocalSourceItem)) (.itemquantity (LocalVariables|GetLocalSourceItem)))
          (CallFunction|CreateNewStack SourceInventory SourceIndex (.itemid (LocalVariables|GetLocalTargetItem)) (.itemquantity (LocalVariables|GetLocalTargetItem))))))
    (:then_1
      (CallFunction|UpdateInventory)
      (CallFunction|UpdateInventory SourceInventory)
      (CallFunction|PlayItemSound (.ItemID (Utilities|Struct|BreakS_InventorySlot (LocalVariables|GetLocalSourceItem)))))))

(fn SplitStack
  (params (Index :type Integer) (SplitQuantity :type Integer))
  (bind (_array_index _found) (CallFunction|SlotsAvailable))
  (bind _inventoryslots (Variables|Default|GetInventorySlots))
  (bind _output (Utilities|Array|Get(acopy) _inventoryslots Index))
  (LocalVariables|SetLocalItemID (.itemid _output))
  (LocalVariables|SetLocalItemQuantity (.itemquantity _output))
  (Utilities|FlowControl|Sequence
    (:then_0
      (if _found
        (LocalVariables|SetLocalAvailableIndex _array_index)
        (if (or (!= SplitQuantity (LocalVariables|GetLocalItemQuantity)) (!= (LocalVariables|GetLocalItemQuantity) 1))
          (CallFunction|CreateNewStack Index (LocalVariables|GetLocalItemID) (- (LocalVariables|GetLocalItemQuantity) SplitQuantity))
          (CallFunction|CreateNewStack (LocalVariables|GetLocalAvailableIndex) (LocalVariables|GetLocalItemID) SplitQuantity))))
    (:then_1
      (CallFunction|PlayItemSound (LocalVariables|GetLocalItemID))
      (CallFunction|UpdateInventory))))

(fn ReturnItems
  (params (SourceInventory :type BPC%20Inventory%20Object%20Reference))
  (bind _inventoryslots (Variables|BPC_Inventory_C|GetInventorySlots SourceInventory))
  (bind _array_element (Utilities|Array|ForEachLoopwithBreak (Variables|BPC_Inventory_C|GetInventorySlots SourceInventory))
    (:LoopBody
      (if (!= (.ItemID (Utilities|Struct|BreakS_InventorySlot _array_element)) "")
        (CallFunction|AddtoInventory (.ItemID (Utilities|Struct|BreakS_InventorySlot _array_element)) (.ItemQuantity (Utilities|Struct|BreakS_InventorySlot _array_element)))))
    (:Completed
      (Utilities|Array|Clear _inventoryslots)
      (Utilities|Array|Resize _inventoryslots (Variables|BPC_Inventory_C|GetInventorySize SourceInventory))
      (CallFunction|UpdateInventory SourceInventory)
      (return))))

(fn GetInventoryValue
  (for _array_element (Variables|Default|GetInventorySlots)
    (if (!= (.ItemID (Utilities|Struct|BreakS_InventorySlot _array_element)) "")
      (LocalVariables|SetLocalTotalValue (+ (LocalVariables|GetLocalTotalValue) (* (.ItemValue (Utilities|Struct|BreakS_ItemDetails (CallFunction|GetItemDetails (.ItemID (Utilities|Struct|BreakS_InventorySlot _array_element))))) (.ItemQuantity (Utilities|Struct|BreakS_InventorySlot _array_element)))))))
  (return (LocalVariables|GetLocalTotalValue)))

(fn FilterOutandReturn
  (bind _outrownames (DataTable|GetDataTableRowNames "/Game/GameAssets/Blueprints/Inventory/ItemData/DataTables/DT_ItemData.DT_ItemData"))
  (for _array_element _outrownames
    (if (and (not (Utilities|Array|ContainsItem (Variables|Default|GetItemsToFilterOut) _array_element)) (!= _array_element "Ichor"))
      (Utilities|Array|AddUnique (LocalVariables|GetLocalFilteredItems) _array_element)))
  (return (LocalVariables|GetLocalFilteredItems)))

(fn GenerateItems
  (bind _addgold (Variables|Default|GetAddGold))
  (Utilities|Array|Clear (Variables|Default|GetInventorySlots))
  (Utilities|Array|Resize (Variables|Default|GetInventorySlots) (Variables|Default|GetInventorySize))
  (Utilities|Array|SetArrayElem (Variables|Default|GetInventorySlots) 0 (Utilities|Struct|MakeS_InventorySlot (Utilities|String|SelectName "Ichor" "None" _addgold) (Math|Integer|SelectInt (Variables|Default|GetIchorAmount) 0 _addgold)))
  (bind _items (CallFunction|FilterOutandReturn))
  (LocalVariables|SetLocalItems _items)
  (for _index (range 1 (Variables|Default|GetItemAmount))
    (if (!= (.OutItem (Utilities|Array|Random (LocalVariables|GetLocalItems))) "")
      (CallFunction|AddtoInventory (.OutItem (Utilities|Array|Random (LocalVariables|GetLocalItems))) (Math|Random|RandomIntegerinRange 1 (.ItemStackSize (Utilities|Struct|BreakS_ItemDetails (CallFunction|GetItemDetails (.OutItem (Utilities|Array|Random (LocalVariables|GetLocalItems)))))))))))

(fn PlayItemSound
  (params (Item :type Name))
  (Audio|PlaySoundatLocation (.Sound (Utilities|Struct|BreakS_ItemDetails (CallFunction|GetItemDetails Item))) (Transformation|GetActorLocation (Components|GetOwner)) "0, 0, 0" 0.1 1.0 0.0 0 0 0 0))