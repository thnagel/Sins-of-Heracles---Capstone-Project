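; Interactable shrine prop that shows a "Pray" prompt and toggles a shrine menu when the player interacts with it.
; The menu widget is created lazily and reused; opening and closing switch input mode, mouse cursor and the player's InPauseMenu flag, which drives the toggle.
; Interacting also adjusts the shimmering audio volume and plays an opening sound.
; Ending overlap with the sphere closes the menu if the widget exists.
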(event OnComponentEndOverlap(SphereCollision)
  (params (OverlappedComponent :type Primitive%20Component%20Object%20Reference) (OtherActor :type Actor%20Object%20Reference) (OtherComp :type Primitive%20Component%20Object%20Reference) (OtherBodyIndex :type Integer))
  ;[0.15 0.15 0.15 0.5] Leaving zone
  (Variables|Default|GetWBP_ShrineMenu
    (:then
      (CallFunction|CloseMenu))
    (:else)))

(event EventInteractwith
  (params (Interactor :type Actor%20Object%20Reference))
  ;[0.15 0.15 0.15 0.5] Open/Close Menu
  (if (Variables|/Game/GameAssets/Blueprints/Player/BP_Player.BP_Player_C|GetinPauseMenu (Variables|Default|GetAs%20BP%20Player))
    (CallFunction|CloseMenu)
    (Audio|Components|Audio|SetVolumeMultiplier (Variables|Default|GetShimmeringAudio) 0.5 :!class /Script/Engine.AudioComponent)
    (else
      (CallFunction|OpenMenu)
      (Audio|PlaySound2D "/Game/GameAssets/Blueprints/Props/Shrine/Audio/ShrimeOpening.ShrimeOpening" 1.0 1.0 0.0 0 0)
      (Audio|Components|Audio|SetVolumeMultiplier (Variables|Default|GetShimmeringAudio) 0.15 :!class /Script/Engine.AudioComponent))))

(event EventBeginPlay
  (bind _asbp_player (Utilities|Casting|CastToBP_Player (Game|Player|GetPlayerPawn 0)))
  (Variables|Default|SetAs%20BP%20Player _asbp_player))

(fn ConstructionScript)

(fn GetShrineMenu
  (Variables|Default|GetWBP_ShrineMenu
    (:then
      _)
    (:else
      (bind _returnvalue (UserInterface|CreateWidget "/Game/GameAssets/Blueprints/Props/Shrine/UI/WBP_ShrineMenu.WBP_ShrineMenu_C" (Game|GetPlayerController 0) 0))
      (bind _output_get (Variables|Default|SetWBP_ShrineMenu _returnvalue))))
  (return _output_get))

(fn OpenMenu
  (bind _returnvalue (Game|GetPlayerController 0))
  (UserInterface|Viewport|AddtoViewport (CallFunction|GetShrineMenu) 0)
  (Input|SetInputModeGameandUI _returnvalue (Variables|Default|GetWBP_ShrineMenu) "DoNotLock" true false)
  (Variables|/Script/Engine.PlayerController|SetbShowMouseCursor _returnvalue true)
  (Variables|/Game/GameAssets/Blueprints/Player/BP_Player.BP_Player_C|SetinPauseMenu (Variables|Default|GetAs%20BP%20Player) true))

(fn CloseMenu
  (bind _returnvalue (Game|GetPlayerController 0))
  (Widget|RemovefromParent (Variables|Default|GetWBP_ShrineMenu))
  (Input|SetInputModeGameOnly _returnvalue false)
  (Variables|/Script/Engine.PlayerController|SetbShowMouseCursor _returnvalue false)
  (Variables|/Game/GameAssets/Blueprints/Player/BP_Player.BP_Player_C|SetinPauseMenu (Variables|Default|GetAs%20BP%20Player) false))

(fn Lookat
  (return "Pray"))