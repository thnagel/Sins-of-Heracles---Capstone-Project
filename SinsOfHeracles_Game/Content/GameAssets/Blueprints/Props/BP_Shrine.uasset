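; Shrine prop the player prays at to open a menu for leveling up and raising stats.
; Interacting toggles a cached WBP_ShrineMenu and its input mode; leaving the sphere closes it.
; LevelUp calls PayIchor to deduct inventory Ichor, plays effects, increments Level and raises Cost inside the VFX cleanup loop; Level rises even when Ichor is insufficient.
; IncreaseStats forwards attribute increases to the player's statistics component.
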(event OnComponentEndOverlap(SphereCollision)
  (params (OverlappedComponent :type Primitive%20Component%20Object%20Reference) (OtherActor :type Actor%20Object%20Reference) (OtherComp :type Primitive%20Component%20Object%20Reference) (OtherBodyIndex :type Integer))
  ;[0.15 0.15 0.15 0.5] Leaving zone
  (Variables|Default|GetWBP_ShrineMenu
    (:then
      (CallFunction|CloseMenu))
    (:else)))

(event Custom|LevelUp
  (bind _returnvalue (Game|GetPlayerCharacter 0))
  (bind _mesh (Variables|/Script/Engine.Character|GetMesh _returnvalue))
  (bind _asbp_player (Utilities|Casting|CastToBP_Player _returnvalue))
  (CallFunction|PayIchor (Variables|/Game/GameAssets/Blueprints/Player/BP_Player.BP_Player_C|GetBPC_Inventory _asbp_player))
  ;[0.15 0.15 0.15 0.5] Handle sfx and vfx
  (bind _returnvalue_2 (Niagara|SpawnSystemAttached "/Game/GameAssets/Blueprints/Props/Shrine/NS_LevelUp.NS_LevelUp" _mesh "None" "0, 0, 0" "0, 0, 0" "KeepRelativeOffset" true))
  (Utilities|Array|Add (Variables|Default|GetVFX) _returnvalue_2)
  (Audio|SpawnSoundAttached "/Game/GameAssets/Blueprints/Props/Shrine/level_up.level_up" _mesh "None" "0, 0, 0" "0, 0, 0" "KeepRelativeOffset" false 1.0 1.0 0.0 0 0)
  (Math|Integer|IncrementInt (Variables|/Game/GameAssets/Blueprints/Player/BPC_Statistics.BPC_Statistics_C|GetLevel (Variables|/Game/GameAssets/Blueprints/Player/BP_Player.BP_Player_C|GetBPC_Statistics (Variables|Default|GetAs%20BP%20Player)))
    (:%20%20
      ;[0.15 0.15 0.15 0.5] Destroy vfx
      (for _array_element (Variables|Default|GetVFX)
        (Components|DestroyComponent _array_element)
        (Variables|Default|SetCost (+ (Variables|Default|GetCost) (* (Math|Conversions|ToFloat(Integer) (Variables|Default|GetCost)) (Variables|Default|GetCostIncrease)))))
      (Variables|Default|SetVFX (Utilities|Array|MakeArray)))))

(event EventInteractwith
  (params (Interactor :type Actor%20Object%20Reference))
  ;[0.15 0.15 0.15 0.5] Open/Close Menu
  (if (Variables|/Game/GameAssets/Blueprints/Player/BP_Player.BP_Player_C|GetinPauseMenu (Variables|Default|GetAs%20BP%20Player))
    (CallFunction|CloseMenu)
    (else
      (CallFunction|OpenMenu)
      (Audio|PlaySound2D "/Game/GameAssets/Blueprints/Props/ShrimeOpening.ShrimeOpening" 1.0 1.0 0.0 0 0))))

(event EventBeginPlay
  (bind _asbp_player (Utilities|Casting|CastToBP_Player (Game|Player|GetPlayerPawn 0)))
  (Variables|Default|SetAs%20BP%20Player _asbp_player))

(fn ConstructionScript)

(fn GetShrineMenu
  (Variables|Default|GetWBP_ShrineMenu
    (:then
      _)
    (:else
      (bind _returnvalue (UserInterface|CreateWidget "/Game/GameAssets/Blueprints/Props/WBP_ShrineMenu.WBP_ShrineMenu_C" (Game|GetPlayerController 0) self))
      (bind _output_get (Variables|Default|SetWBP_ShrineMenu _returnvalue))))
  (return _output_get))

(fn OpenMenu
  (bind _returnvalue (Game|GetPlayerController 0))
  (UserInterface|Viewport|AddtoViewport (CallFunction|GetShrineMenu) 0)
  (Input|SetInputModeGameandUI _returnvalue (Variables|Default|GetWBP_ShrineMenu) "DoNotLock" true false)
  (Variables|/Script/Engine.PlayerController|SetbShowMouseCursor _returnvalue true)
  (Variables|/Game/GameAssets/Blueprints/Player/BP_Player.BP_Player_C|SetinPauseMenu (Variables|Default|GetAs%20BP%20Player) true))

(fn CloseMenu
  (bind _returnvalue (Game|GetPlayerController 0))
  (Widget|RemovefromParent (Variables|Default|GetWBP_ShrineMenu))
  (Input|SetInputModeGameOnly _returnvalue false)
  (Variables|/Script/Engine.PlayerController|SetbShowMouseCursor _returnvalue false)
  (Variables|/Game/GameAssets/Blueprints/Player/BP_Player.BP_Player_C|SetinPauseMenu (Variables|Default|GetAs%20BP%20Player) false))

(fn IncreaseStats
  (params (Strength :type Integer) (Dexterity :type Integer) (Vitality :type Integer) (Endurance :type Integer))
  (bind _as_bp_player (Variables|Default|GetAs%20BP%20Player))
  (bind _bpc_statistics (Variables|/Game/GameAssets/Blueprints/Player/BP_Player.BP_Player_C|GetBPC_Statistics _as_bp_player))
  (Default|IncreaseStrength _bpc_statistics Strength)
  (Default|IncreaseDexterity _bpc_statistics Dexterity)
  (Default|IncreaseVitality _bpc_statistics Vitality)
  (Default|IncreaseEndurance _bpc_statistics Endurance))

(fn PayIchor
  (params (PlayerInventory :type BPC%20Inventory%20Object%20Reference))
  (bind _cost (Variables|Default|GetCost))
  (bind _inventoryslots (Variables|/Game/GameAssets/Blueprints/Inventory/BPC_Inventory.BPC_Inventory_C|GetInventorySlots PlayerInventory))
  (if (>= (Variables|/Game/GameAssets/Blueprints/Inventory/BPC_Inventory.BPC_Inventory_C|GetIchorAmount PlayerInventory) _cost)
    ;[0.15 0.15 0.15 0.5] Look for the slot containing ichor
    (bind (_array_element _array_index) (Utilities|Array|ForEachLoopwithBreak _inventoryslots)
      (:LoopBody
        (if (== (.itemid _array_element) "Ichor")
          (Variables|Default|SetIchorIndex _array_index)))
      (:Completed
        ;[0.15 0.15 0.15 0.5] Reduce the ammount of ichor in the found  slot
        (Utilities|Array|SetArrayElem _inventoryslots (Variables|Default|GetIchorIndex) (Utilities|Struct|MakeS_InventorySlot (.itemid (Utilities|Array|Get(acopy) _inventoryslots (Variables|Default|GetIchorIndex))) (- (.itemquantity (Utilities|Array|Get(acopy) _inventoryslots (Variables|Default|GetIchorIndex))) _cost)))
        (Variables|/Game/GameAssets/Blueprints/Inventory/BPC_Inventory.BPC_Inventory_C|SetIchorAmount PlayerInventory (- (.itemquantity (Utilities|Array|Get(acopy) _inventoryslots (Variables|Default|GetIchorIndex))) _cost))
        (Default|UpdateInventory PlayerInventory)))))

(fn Lookat
  (return "Pray"))