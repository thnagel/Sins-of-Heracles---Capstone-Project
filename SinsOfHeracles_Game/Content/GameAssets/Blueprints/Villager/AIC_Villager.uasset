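; AI controller for villagers that wanders a level by alternating between waypoint travel and random roaming.
; On BeginPlay it waits a tick, caches all BP_Waypoint actors and moves to a random one.
; Arrival triggers a pause and coin flip between roaming and another waypoint, while failure retries immediately.
; Roaming targets a nearby navigable point, then randomly re-rolls or returns to waypoints on short delays without awaiting arrival.
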(event Custom|WaypointMovement
  ;[0.15 0.15 0.15 0.5] Basic Waypoint Movement
  (AI|AIMoveTo (Pawn|GetControlledPawn) "0, 0, 0" (Utilities|Array|Get(acopy) (Variables|Default|GetWaypoints) (Math|Random|RandomIntegerinRange 0 (- (Utilities|Array|Length (Variables|Default|GetWaypoints)) 1))) 5e+02 false
    (:OnSuccess
      (Utilities|FlowControl|Delay 2.0)
      (if (Math|Random|RandomBool)
        (CallFunction|RoamMovement)
        (else
          (CallFunction|WaypointMovement))))
    (:OnFail
      (CallFunction|WaypointMovement))))

(event Custom|RoamMovement
  ;[0.15 0.15 0.15 0.5] Basic Roam movement
  (bind _randomlocation (Class|NavigationSystemV1|GetRandomLocationinNavigableRadius (Transformation|GetActorLocation (Pawn|GetControlledPawn)) (Variables|Default|GetRoamRadius) 0 0))
  (AI|AIMoveTo 0 _randomlocation 0 -1.0 "Default" "Default" true true
    (:then
      (if (Math|Random|RandomBool)
        (Utilities|FlowControl|Delay 1.0)
        (CallFunction|RoamMovement)
        (else
          (Utilities|FlowControl|Delay 2.5)
          (CallFunction|WaypointMovement))))))

(event EventBeginPlay
  ;[0.15 0.15 0.15 0.5] Get all waypoints
  (Utilities|FlowControl|DelayUntilNextTick)
  (bind _outactors (Actor|GetAllActorsOfClass "/Game/GameAssets/Blueprints/Villager/BP_Waypoint.BP_Waypoint_C"))
  (Variables|Default|SetWaypoints _outactors)
  (CallFunction|WaypointMovement))

(fn ConstructionScript)