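; Villager character that steps away when the player gets close, then resumes its AI-driven movement.
; BeginPlay caches the player and its AIC_Villager controller and sets walk speed from TargetSpeed.
; When the player overlaps SphereCollision, AIMoveTo sends it to a point directly away from the player.
; On a successful move, it waits briefly, then randomly calls the controller's WaypointMovement or RoamMovement.
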(event OnComponentBeginOverlap(SphereCollision)
  (params (OverlappedComponent :type Primitive%20Component%20Object%20Reference) (OtherActor :type Actor%20Object%20Reference) (OtherComp :type Primitive%20Component%20Object%20Reference) (OtherBodyIndex :type Integer) (bFromSweep :type Boolean) (SweepResult :type Hit%20Result%20Structure%20%28by%20ref%29))
  (if (== OtherActor (Variables|Default|GetAs%20BP%20Player))
    (AI|AIMoveTo self (+ (Transformation|GetActorLocation) (* (Math|Vector|Normalize (- (Transformation|GetActorLocation) (Transformation|GetActorLocation (Variables|Default|GetAs%20BP%20Player)))) 5e+02)) 0 5e+01 false
      (:OnSuccess
        (Utilities|FlowControl|Delay 1.0)
        (if (Math|Random|RandomBool)
          (Default|WaypointMovement (Variables|Default|GetAs%20AIC%20Villager))
          (else
            (Default|RoamMovement (Variables|Default|GetAs%20AIC%20Villager))))))))

(event EventBeginPlay
  ;[0.15 0.15 0.15 0.5] Setup walk speed and useful refs
  (bind _asbp_player (Utilities|Casting|CastToBP_Player (Game|GetPlayerCharacter 0)))
  (Variables|Default|SetAs%20BP%20Player _asbp_player)
  (bind _asaic_villager (Utilities|Casting|CastToAIC_Villager (Pawn|GetController)))
  (Variables|Default|SetAs%20AIC%20Villager _asaic_villager)
  (Variables|/Script/Engine.CharacterMovementComponent|SetMaxWalkSpeed (Variables|Character|GetCharacterMovement) (Variables|Default|GetTargetSpeed)))

(fn ConstructionScript)