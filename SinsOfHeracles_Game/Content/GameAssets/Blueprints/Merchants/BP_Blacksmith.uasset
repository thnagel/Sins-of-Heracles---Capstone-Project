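; BP_Blacksmith is an interactable blacksmith merchant that shows "Forge" as its look-at text.
; Interacting opens a dialogue through its dialogue component, unless the player is already in a menu.
; OpenMenu toggles the blacksmith menu widget, switching input mode, cursor and the player's InPauseMenu flag.
; Leaving the sphere collision shares the toggle's closing path, which removes the menu, restores game input and ends dialogue.
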(event OnComponentEndOverlap(SphereColision)
  (params (OverlappedComponent :type Primitive%20Component%20Object%20Reference) (OtherActor :type Actor%20Object%20Reference) (OtherComp :type Primitive%20Component%20Object%20Reference) (OtherBodyIndex :type Integer))
  (bind _returnvalue (Game|GetPlayerController 0))
  (bind _ui (Variables|Default|GetUI))
  (if (== OtherActor (Game|GetPlayerCharacter 0))
    (Utilities|IsValid _ui
      (:Is%20Valid
        (Widget|RemovefromParent _ui))
      (:Is%20Not%20Valid
        _))
    (Input|SetInputModeGameOnly _returnvalue false)
    (Variables|/Script/Engine.PlayerController|SetbShowMouseCursor _returnvalue false)
    (Variables|/Game/GameAssets/Blueprints/Player/BP_Player.BP_Player_C|SetinPauseMenu (Variables|Default|GetAs%20BP%20Player) false)
    (Default|EndDialogue (Variables|Default|GetBPC_Dialogue))
    (CallFunction|HideMouse)))

(event Custom|OpenMenu
  (bind _returnvalue (Game|GetPlayerController 0))
  (bind _as_bp_player (Variables|Default|GetAs%20BP%20Player))
  (if (Variables|/Game/GameAssets/Blueprints/Player/BP_Player.BP_Player_C|GetinPauseMenu _as_bp_player)
    (Utilities|IsValid (Variables|Default|GetUI)
      (:Is%20Valid
        (Widget|RemovefromParent (Variables|Default|GetUI)))
      (:Is%20Not%20Valid
        _))
    (Input|SetInputModeGameOnly _returnvalue false)
    (Variables|/Script/Engine.PlayerController|SetbShowMouseCursor _returnvalue false)
    (Variables|/Game/GameAssets/Blueprints/Player/BP_Player.BP_Player_C|SetinPauseMenu (Variables|Default|GetAs%20BP%20Player) false)
    (Default|EndDialogue (Variables|Default|GetBPC_Dialogue))
    (CallFunction|HideMouse)
    (else
      (bind _returnvalue_2 (UserInterface|CreateWidget "/Game/GameAssets/Blueprints/Merchants/UI/WBP_BlacksmithMenu.WBP_BlacksmithMenu_C" 0 _as_bp_player))
      (bind _output_get (Variables|Default|SetUI _returnvalue_2))
      (UserInterface|Viewport|AddtoViewport _output_get 0)
      (Input|SetInputModeGameandUI (Game|GetPlayerController 0) _output_get "DoNotLock" true false)
      (Variables|/Script/Engine.PlayerController|SetbShowMouseCursor (Game|GetPlayerController 0) true)
      (Variables|/Game/GameAssets/Blueprints/Player/BP_Player.BP_Player_C|SetinPauseMenu (Variables|Default|GetAs%20BP%20Player) true))))

(event EventInteractwith
  (params (Interactor :type Actor%20Object%20Reference))
  (if (not (Variables|/Game/GameAssets/Blueprints/Player/BP_Player.BP_Player_C|GetinPauseMenu (Variables|Default|GetAs%20BP%20Player)))
    (Default|CreateDialogDisplay (Variables|Default|GetBPC_Dialogue))))

(event EventBeginPlay
  (bind _asbp_player (Utilities|Casting|CastToBP_Player (Game|Player|GetPlayerPawn 0)))
  (Variables|Default|SetAs%20BP%20Player _asbp_player))

(fn ConstructionScript)

(fn Lookat
  (return "Forge"))