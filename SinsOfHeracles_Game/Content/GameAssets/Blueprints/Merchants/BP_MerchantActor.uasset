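; BP_MerchantActor is a merchant actor that settles item trades between a merchant inventory and the player's inventory.
; It handles two trade events, each receiving the merchant's inventory and fetching the player's through GetPlayerInventory.
; Cancelling returns MerchantOffer and PlayerOffer to their original owners, while accepting swaps them, using the same ReturnItems call in both cases.
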(event Custom|TradeAccepted
  (params (MerchantInventory :type BPC%20Inventory%20Object%20Reference))
  (Default|ReturnItems MerchantInventory (Variables|Default|GetPlayerOffer))
  (bind _playerinventory (CallFunction|GetPlayerInventory))
  (Default|ReturnItems _playerinventory (Variables|Default|GetMerchantOffer)))

(event Custom|TradeCancelled
  (params (MerchantInventory :type BPC%20Inventory%20Object%20Reference))
  (Default|ReturnItems MerchantInventory (Variables|Default|GetMerchantOffer))
  (bind _playerinventory (CallFunction|GetPlayerInventory))
  (Default|ReturnItems _playerinventory (Variables|Default|GetPlayerOffer)))

(event EventBeginPlay)

(fn ConstructionScript)