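; BPC_Merchant is a merchant component that toggles a trading session for a given inventory component.
; Opening spawns a BP_MerchantActor and creates a WBP_TradeView linked to the inventory, actor and component, then plays its PopIn animation.
; Closing cancels the trade, destroys the actor and reverses PopIn, with a looping timer polling until the animation ends before removing the widget.
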(event EventBeginPlay)

(event EventTick
  (params (DeltaSeconds :type Float%20%28single-precision%29)))

(fn SpawnMerchantActor
  (bind _returnvalue (Game|SpawnActorfromClass "/Game/GameAssets/Blueprints/Merchants/BP_MerchantActor.BP_MerchantActor_C" (Math|Transform|MakeTransform "0, 0, 0" "0, 0, 0" "1.000000,1.000000,1.000000") "Undefined" "MultiplyWithRoot" 0 0))
  (Variables|Default|SetMerchantActor _returnvalue))

(fn CreateTradeView
  (bind _returnvalue (UserInterface|CreateWidget "/Game/GameAssets/Blueprints/Merchants/UI/WBP_TradeView.WBP_TradeView_C" 0 (Variables|Default|GetMerchantInventory) (Variables|Default|GetMerchantActor) self))
  (bind _output_get (Variables|Default|SetTradeViewUI _returnvalue))
  (UserInterface|Animation|PlayAnimation _output_get (Variables|/Game/GameAssets/Blueprints/Merchants/UI/WBP_TradeView.WBP_TradeView_C|GetPopIn _output_get) 0.0 1 "Forward" 1.0 false)
  (UserInterface|Viewport|AddtoViewport _output_get 0))

(fn ToggleTrading
  (params (InventoryComponent :type BPC%20Inventory%20Object%20Reference))
  (bind _tradeviewui (Variables|Default|GetTradeViewUI))
  (bind _merchantactor (Variables|Default|GetMerchantActor)
    (:then
      (Default|TradeCancelled _merchantactor (Variables|Default|GetMerchantInventory))
      (Actor|DestroyActor (Variables|Default|GetMerchantActor))
      (Variables|Default|SetMerchantActor 0)
      (UserInterface|Animation|PlayAnimation _tradeviewui (Variables|/Game/GameAssets/Blueprints/Merchants/UI/WBP_TradeView.WBP_TradeView_C|GetPopIn _tradeviewui) 0.0 1 "Reverse" 1.0 false)
      (bind _returnvalue (Utilities|Time|SetTimerbyFunctionName 0 "CheckAnimationDelay" 0.1 true true))
      (Variables|Default|SetAnimEndFuncHandle _returnvalue))
    (:else
      (Variables|Default|SetMerchantInventory InventoryComponent)
      (CallFunction|SpawnMerchantActor)
      (CallFunction|CreateTradeView))))

(fn CheckAnimationDelay
  (bind _tradeviewui (Variables|Default|GetTradeViewUI))
  (if (not (Class|UserWidget|IsAnimationPlaying _tradeviewui (Variables|/Game/GameAssets/Blueprints/Merchants/UI/WBP_TradeView.WBP_TradeView_C|GetPopIn _tradeviewui)))
    (Utilities|Time|ClearandInvalidateTimerbyHandle (Variables|Default|GetAnimEndFuncHandle))
    (Widget|RemovefromParent (Variables|Default|GetTradeViewUI))))