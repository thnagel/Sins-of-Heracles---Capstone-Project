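; BP_Merchant is an interactable merchant that opens trading with its inventory and shows a "Trade" look-at prompt.
; The first interaction after BeginPlay generates items through BPCInventory, and each interaction toggles trading on BPCMerchant with that inventory.
; When an overlap with the collision sphere ends, it toggles trading again if BPCMerchant holds a valid MerchantActor.
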(event OnComponentEndOverlap(SphereColision)
  (params (OverlappedComponent :type Primitive%20Component%20Object%20Reference) (OtherActor :type Actor%20Object%20Reference) (OtherComp :type Primitive%20Component%20Object%20Reference) (OtherBodyIndex :type Integer))
  (Variables|/Game/GameAssets/Blueprints/Merchants/BPC_Merchant.BPC_Merchant_C|GetMerchantActor (Variables|Default|GetBPC_Merchant)
    (:then
      (Default|ToggleTrading (Variables|Default|GetBPC_Merchant) (Variables|Default|GetBPC_Inventory)))
    (:else)))

(event EventBeginPlay
  (Variables|Default|SetIsInvGenerated false))

(event EventInteractwith
  (params (Interactor :type Actor%20Object%20Reference))
  (if (Variables|Default|GetIsInvGenerated)
    _
    (else
      (CallFunction|RerollIMerchantInventory)
      (Variables|Default|SetIsInvGenerated true)))
  (Default|ToggleTrading (Variables|Default|GetBPC_Merchant) (Variables|Default|GetBPC_Inventory)))

(fn ConstructionScript)

(fn RerollIMerchantInventory
  (Default|GenerateItems (Variables|Default|GetBPC_Inventory)))

(fn Lookat
  (return "Trade"))